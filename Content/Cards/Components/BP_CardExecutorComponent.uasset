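; BP_CardExecutorComponent is a component that executes played cards against the player character.
; On BeginPlay it builds a list of processor objects, one for damage and one for healing.
; PlayCard casts the player pawn, prints the card name, then passes the card and character to every processor, so each effect type lives in its own class.
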(event Custom|Event%20Play%20Card
  (params (CardData :type Card%20Object%20Reference))
  (bind _asplayer_character (Utilities|Casting|CastToPlayerCharacter (Game|Player|GetPlayerPawn 0)))
  (Development|PrintText (Utilities|Text|FormatText (Utilities|Text|MakeLiteralText "Play {0}") (Variables|/Script/CS3247_Project.Card|GetName CardData)))
  (for _array_element (Variables|Default|GetProcessors)
    (Class|CardProcessor|ProcessCard _array_element CardData _asplayer_character)))

(event EventBeginPlay
  (bind _processors (Variables|Default|GetProcessors))
  (bind _returnvalue (Game|ConstructObjectfromClass "/Game/Cards/Components/BP_CardDamageProcessor.BP_CardDamageProcessor_C"))
  (Utilities|Array|Add _processors _returnvalue)
  (bind _returnvalue_2 (Game|ConstructObjectfromClass "/Game/Cards/Components/BP_CardHealProcessor.BP_CardHealProcessor_C"))
  (Utilities|Array|Add _processors _returnvalue_2))