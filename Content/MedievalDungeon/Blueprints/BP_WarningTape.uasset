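; BP_WarningTape is a warning tape actor that scrolls two text render components along the world Y axis.
; On BeginPlay it caches both starting locations, then runs a separate timeline for each text, offsetting it in negative Y by the timeline's YMovement track.
; The second timeline starts after a fixed delay, staggering the two texts.
; The first text's width is also stored in TextLength, but nothing in this graph reads it.
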(event EventBeginPlay
  (Variables|Default|SetInitialLocation1 (Transformation|GetWorldLocation (Variables|Default|GetTextRender1)))
  (Variables|Default|SetInitialLocation2 (Transformation|GetWorldLocation (Variables|Default|GetTextRender2)))
  (Variables|Default|SetTextLength (.y (Class|TextRenderComponent|GetTextWorldSize (Variables|Default|GetTextRender1))))
  (Utilities|FlowControl|Sequence
    (:then_0
      (bind _y_movement (Timeline|Play1 Play)
        (:Update
          (Transformation|SetWorldLocation (Variables|Default|GetTextRender1) (- (Variables|Default|GetInitialLocation1) (Math|Vector|MakeVector 0.0 _y_movement 0.0)) false false))))
    (:then_1
      (Utilities|FlowControl|Delay 1e+01)
      (bind _y_movement_2 (Timeline|Play2 Play)
        (:Update
          (Transformation|SetWorldLocation (Variables|Default|GetTextRender2) (- (Variables|Default|GetInitialLocation2) (Math|Vector|MakeVector 0.0 _y_movement_2 0.0)) false false))))))

(fn ConstructionScript)