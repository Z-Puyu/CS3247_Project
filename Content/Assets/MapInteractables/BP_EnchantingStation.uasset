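; BP_EnchantingStation is a map interactable that switches its candles and audio with its active state.
; On BeginPlay it finds its child actors of type BP_EnchantingStationCandle and binds events to the OnActivated and OnDeactivated dispatchers.
; OnActivate and OnDeactivate broadcast those dispatchers, so candles follow without direct calls, and fade the station's audio in or out.
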(event Custom|Event%20On%20Activate
  (Default|CallOnActivated)
  (Audio|Components|Audio|FadeIn (Variables|Default|GetAudio) 2.0 1.0 0.0 "Linear" :!class /Script/Engine.AudioComponent))

(event Custom|Event%20On%20Deactivate
  (Default|CallOnDeactivated)
  (Audio|Components|Audio|FadeOut (Variables|Default|GetAudio) 3.0 0.0 "Linear" :!class /Script/Engine.AudioComponent))

(event EventBeginPlay
  (for _array_element (Actor|GetAllChildActors true)
    (bind _asbp_enchanting_station_candle (Utilities|Casting|CastToBP_EnchantingStationCandle _array_element))
    (EventDispatchers|BindEventtoOnActivated (EventDispatchers|CreateEvent _asbp_enchanting_station_candle :!event EventonLit))
    (EventDispatchers|BindEventtoOnDeactivated (EventDispatchers|CreateEvent _asbp_enchanting_station_candle :!event EventonPutOff))))

(fn ConstructionScript)