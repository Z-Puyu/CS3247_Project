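; BP_TableInteractable is a map interactable that drives a table actor through the open and close states inherited from its parent.
; On BeginPlay it casts the InteractableActor component's child actor to BP_Table and stores the reference.
; Its On Open and On Close overrides run the parent logic, then fire the table's activate and deactivate events respectively.
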(event EventBeginPlay
  (bind _asbp_table (Utilities|Casting|CastToBP_Table (Variables|/Script/Engine.ChildActorComponent|GetChildActor (Variables|Default|GetInteractableActor))))
  (Variables|Default|SetTable _asbp_table))

(fn ConstructionScript
  (|CallParentFunction))

(fn OnOpen
  (|CallParentFunction)
  (Default|EventonActivate (Variables|Default|GetTable)))

(fn OnClose
  (|CallParentFunction)
  (Default|EventonDeactivate (Variables|Default|GetTable)))