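; BP_TreasureChestInteractable is a map interactable that represents an openable and closable treasure chest.
; On BeginPlay it casts the InteractableActor child actor to BP_TreasureChest and caches the reference.
; Its On Open and On Close overrides call the parent logic, then forward to the chest's activated and deactivated events.
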(event EventBeginPlay
  (|CallParentFunction)
  (bind _asbp_treasure_chest (Utilities|Casting|CastToBP_TreasureChest (Variables|/Script/Engine.ChildActorComponent|GetChildActor (Variables|Default|GetInteractableActor))))
  (Variables|Default|SetTreasureChest _asbp_treasure_chest))

(fn ConstructionScript
  (|CallParentFunction))

(fn OnOpen
  (|CallParentFunction)
  (Default|EventonActivated (Variables|Default|GetTreasureChest)))

(fn OnClose
  (|CallParentFunction)
  (Default|EventonDeactivated (Variables|Default|GetTreasureChest)))