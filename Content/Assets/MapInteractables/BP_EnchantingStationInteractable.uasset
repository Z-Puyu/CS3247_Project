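; BP_EnchantingStationInteractable is a map interactable that lets a player in range use an enchanting station.
; On BeginPlay it casts the InteractableActor child actor to BP_EnchantingStation and caches it.
; Range events call the parent handlers, then activate or deactivate the station as the player enters or leaves.
; Pressing the Interact input fires the use-enchanting-station event on the player in range.
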(event EventBeginPlay
  (bind _asbp_enchanting_station (Utilities|Casting|CastToBP_EnchantingStation (Variables|/Script/Engine.ChildActorComponent|GetChildActor (Variables|Default|GetInteractableActor))))
  (Variables|Default|SetEnchantingStation _asbp_enchanting_station))

(event EventOnPlayerinRange
  (params (Player :type Player%20Character%20Object%20Reference))
  (|CallParentFunction Player)
  (Default|EventonActivate (Variables|Default|GetEnchantingStation)))

(event EventOnPlayerOutOfRange
  (params (Player :type Player%20Character%20Object%20Reference))
  (|CallParentFunction Player)
  (Default|EventonDeactivate (Variables|Default|GetEnchantingStation)))

(event Input|ActionEvents|InputActionInteract
  (params (Key :type Key%20Structure :default "None"))
  (:Pressed
    (Default|EventonUseEnchantingStation (Variables|Default|GetPlayerInRange))))

(fn ConstructionScript)