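; Candle actor for the enchanting station that can be lit and put out through OnLit and OnPutoff events.
; It starts with its point light hidden.
; Lighting activates the flame particle, shows the light, plays a one-shot ignition sound at its location and starts its audio component.
; Putting it out deactivates the flame, hides the light and stops the audio.
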(event Custom|Event%20On%20Lit
  (Components|Activation|Activate (Variables|Default|GetFlameParticle) true)
  (Rendering|SetVisibility (Variables|Default|GetPointLight) true false)
  (Audio|PlaySoundatLocation "/Game/Audio/SFX/MapObjects/Candle_Light_Up_Cue.Candle_Light_Up_Cue" (Transformation|GetActorLocation) "0, 0, 0" 1.0 1.0 0.0 0 0 0 0)
  (Audio|Components|Audio|Play (Variables|Default|GetAudio) 0.0))

(event Custom|Event%20On%20Put%20off
  (Components|Activation|Deactivate (Variables|Default|GetFlameParticle))
  (Rendering|SetVisibility (Variables|Default|GetPointLight) false false)
  (Audio|Components|Audio|Stop (Variables|Default|GetAudio)))

(event EventBeginPlay
  (Rendering|SetVisibility (Variables|Default|GetPointLight) false false))

(fn ConstructionScript)