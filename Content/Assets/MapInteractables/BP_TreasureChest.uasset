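; BP_TreasureChest is an interactable treasure chest whose lid swings open when activated and shut when deactivated.
; OnActivated plays the open sound at the chest and runs the LidMoving timeline forward, scaling its Opening track into ChestLid's relative roll.
; OnDeactivated plays the close sound and drives the same roll through a second timeline, reversed from the end, rather than reversing LidMoving.
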(event Custom|Event%20On%20Activated
  (Audio|PlaySoundatLocation "/Game/Audio/SFX/MapObjects/Chest_Open_Cue.Chest_Open_Cue" (Transformation|GetActorLocation) "0, 0, 0" 1.0 1.0 0.0 0 0 0 0)
  (bind _opening (Timeline|LidMoving PlayFromStart)
    (:Update
      (Transformation|SetRelativeRotation (Variables|Default|GetChestLid) (Math|Rotator|MakeRotator (* _opening -45.0) 0.0 0.0) false false))))

(event Custom|Event%20On%20Deactivated
  (Audio|PlaySoundatLocation "/Game/Audio/SFX/MapObjects/Close_Chest_Cue.Close_Chest_Cue" (Transformation|GetActorLocation) "0, 0, 0" 1.0 1.0 0.0 0 0 0 0)
  (bind _opening (Timeline|Timeline ReverseFromEnd)
    (:Update
      (Transformation|SetRelativeRotation (Variables|Default|GetChestLid) (Math|Rotator|MakeRotator (* _opening -45.0) 0.0 0.0) false false))))

(fn ConstructionScript)