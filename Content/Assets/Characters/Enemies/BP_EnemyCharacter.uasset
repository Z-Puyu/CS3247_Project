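; Data-driven enemy for a turn-based dungeon game, shown as a Paper2D sprite with highlight tint and a status widget.
; BeginPlay async-loads the sprite and ash meshes, seeds GAS attributes from EnemyData via set-by-caller effects, and relays attribute changes.
; On its turn, Utility AI picks skill effects and targets, broadcast as actions with matching sounds.
; At zero health it spawns remains carrying random loot and broadcasts death.
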(event Custom|Event%20On%20Disable%20Highlight
  (Sprite|SetSpriteColor (Variables|Default|GetSprite) (Utilities|Struct|MakeLinearColor 1.0 1.0 1.0 1.0)))

(event Custom|Event%20On%20Enable%20Highlight
  (Sprite|SetSpriteColor (Variables|Default|GetSprite) (Variables|Default|GetHighlight)))

(event Custom|Event%20On%20Defeated
  (bind _returnvalue (Transformation|GetActorTransform))
  (bind (_location _rotation _scale) (Math|Transform|BreakTransform _returnvalue))
  (bind _returnvalue_2 (* _location "1.000000,1.000000,0.000000"))
  (bind _loots (CallFunction|DropLoots))
  (Game|SpawnActorfromClass "/Game/Assets/Characters/Enemies/BP_EnemyRemains.BP_EnemyRemains_C" (Math|Transform|MakeTransform _returnvalue_2 _rotation _scale) "AlwaysSpawn" "MultiplyWithRoot" 0 _loots (Utilities|ResolveSoftReference (.OutItem (Utilities|Array|Random (Variables|Default|GetAshMeshes)))) 0)
  (Variables|Default|SetbIsDead true)
  (Audio|PlaySoundatLocation "/Game/Audio/SFX/Combat/Enemy_Dies_Cue.Enemy_Dies_Cue" _returnvalue_2 "0, 0, 0" 1.0 1.0 0.0 0 0 0 0)
  (Default|CallOnDeath))

(event Custom|Event%20On%20Init%20Attribute
  (params (Attribute :type Gameplay%20Attribute%20Structure) (Value :type Float%20%28double-precision%29))
  (bind _returnvalue (Ability|GetAbilitySystemComponent 0))
  (bind _asbp_dungeon_slayer_game_instance (Utilities|Casting|CastToBP_DungeonSlayerGameInstance (Game|GetGameInstance)))
  (bind _returnvalue_2 (Class|BasicGameInstance|AttributetoAssetTag _asbp_dungeon_slayer_game_instance Attribute))
  (bind _returnvalue_3 (Ability|GameplayEffect|AssignTagSetbyCallerMagnitude (GameplayEffects|MakeOutgoingSpec :self _returnvalue :GameplayEffectClass "/Game/Assets/GameplayAbilities/GameplayEffects/GE_InitAttribute.GE_InitAttribute_C" :Level 1.0) "(TagName=\"GameplayEffect.AttributeInitialisation\")" Value))
  (bind _returnvalue_4 (Ability|GameplayEffect|AddAssetTag _returnvalue_3 _returnvalue_2))
  (GameplayEffects|ApplyGameplayEffectSpecToSelf _returnvalue _returnvalue_4))

(event Custom|Event%20On%20Attribute%20Updated
  (params (Attribute :type Gameplay%20Attribute%20Structure) (OldValue :type Integer) (CurrentValue :type Integer))
  (if (== Attribute "(AttributeName=\"Health\",Attribute=/Script/CS3247_Project.BasicAttributeSet:Health,AttributeOwner=\"/Script/CoreUObject.Class'/Script/CS3247_Project.BasicAttributeSet'\")")
    (Default|CallOnAttributeDataUpdated Attribute CurrentValue (Math|Float|Truncate (.CurrentValue (Utilities|Struct|BreakGameplayAttributeData (Variables|/Script/CS3247_Project.BasicAttributeSet|GetMaxHealth (Variables|Default|GetAttributeSet))))))
    (if (<= CurrentValue 0)
      (CallFunction|EventonDefeated))
    (else
      (Default|CallOnAttributeDataUpdated Attribute CurrentValue))))

(event EventBeginPlay
  (bind _enemydata (Variables|Default|GetEnemyData))
  (bind _attributes (Variables|/Script/CS3247_Project.Enemy|GetAttributes _enemydata))
  (bind _object (Utilities|AsyncLoadAsset (Variables|/Script/CS3247_Project.Enemy|GetSprite (Variables|Default|GetEnemyData)))
    (:then
      (for _array_element (Variables|Default|GetAshMeshes)
        (Utilities|AsyncLoadAsset _array_element))
      (bind _keys (Utilities|Map|Keys _attributes))
      (for _array_element_2 _keys
        (CallFunction|EventonInitAttribute _array_element_2 (.Value (Utilities|Map|Find _attributes _array_element_2))))
      (bind _aswbp_enemy_health_display (Utilities|Casting|CastToWBP_EnemyHealthDisplay (UserInterface|GetWidget (Variables|Default|GetEnemyStatusWidget))))
      (Rendering|Components|TextRender|SetText (Variables|/Game/UI/Combat/WBP_EnemyHealthDisplay.WBP_EnemyHealthDisplay_C|GetName _aswbp_enemy_health_display) (Utilities|Text|ToText(Name) (Variables|/Script/CS3247_Project.Enemy|GetName (Variables|Default|GetEnemyData))))
      (EventDispatchers|BindEventtoOnAttributeDataUpdated (EventDispatchers|CreateEvent _aswbp_enemy_health_display :!event EventonAttributesUpdated))
      (EventDispatchers|BindEventtoOnAttributeChanged (Variables|Default|GetAttributeSet) (delegate Custom|Event%20On%20Attribute%20Updated)))
    (:Completed
      (bind _aspaper_sprite (Utilities|Casting|CastToPaperSprite _object))
      (Rendering|Components|Sprite|SetSprite (Variables|Default|GetSprite) _aspaper_sprite))))

(event Custom|Event%20On%20Use%20Skill
  (params (GameplayEffects :type Array%20of%20Gameplay%20Effect%20Descriptor%20Structures) (TargetCharacter :type Array%20of%20Basic%20Character%20Object%20References))
  (for _array_element GameplayEffects
    (for _array_element_2 TargetCharacter
      (Default|CallOnActionTaken _array_element_2 self 1.0 _array_element))
    (CallFunction|EventonPlayAttackSound _array_element)
    (CallFunction|EventonPlayDefendSound _array_element)
    (CallFunction|EventonPlayHealSound _array_element)))

(event Custom|Event%20On%20Take%20Action
  (params (Context :type Combat%20Context%20Structure))
  (bind _utilityai (Variables|Default|GetUtilityAi))
  (bind _returnvalue (Class|UtilityAiComponent|Decide _utilityai Context))
  (bind (_skilleffects _targets) (Utilities|Struct|BreakAiDecision _returnvalue))
  (CallFunction|EventonUseSkill _skilleffects _targets))

(event Custom|Event%20On%20Play%20Defend%20Sound
  (params (GameplayEffect :type Gameplay%20Effect%20Descriptor%20Structure))
  (if (== (.GameplayEffectType (Utilities|Struct|BreakGameplayEffectDescriptor GameplayEffect)) "/Game/Assets/GameplayAbilities/GameplayEffects/GE_Defend.GE_Defend_C")
    (Audio|PlaySound2D "/Game/Audio/SFX/Combat/Defend_Cue.Defend_Cue" 1.0 1.0 0.0 0 0 false)))

(event Custom|Event%20On%20Play%20Attack%20Sound
  (params (GameplayEffect :type Gameplay%20Effect%20Descriptor%20Structure))
  (if (== (.GameplayEffectType (Utilities|Struct|BreakGameplayEffectDescriptor GameplayEffect)) "/Game/Assets/GameplayAbilities/GameplayEffects/GE_Damage.GE_Damage_C")
    (Audio|PlaySound2D "/Game/Audio/SFX/Combat/Attacked_by_Enemy.Attacked_by_Enemy" 1.0 1.0 0.0 0 0 false)))

(event Custom|Event%20On%20Play%20Heal%20Sound
  (params (GameplayEffect :type Gameplay%20Effect%20Descriptor%20Structure))
  (if (== (.GameplayEffectType (Utilities|Struct|BreakGameplayEffectDescriptor GameplayEffect)) "/Game/Assets/GameplayAbilities/GameplayEffects/GE_Healing.GE_Healing_C")
    (Audio|PlaySound2D "/Game/Audio/SFX/Combat/Enemy_Heal.Enemy_Heal" 1.0 1.0 0.0 0 0 false)))

(fn ConstructionScript)

(fn DropLoots
  (bind _enemydata (Variables|Default|GetEnemyData))
  (bind _possibleloots (Variables|/Script/CS3247_Project.Enemy|GetPossibleLoots _enemydata))
  (bind _outitem (Utilities|Array|Random _possibleloots))
  (bind (_item _minquantity _maxquantity) (Utilities|Struct|BreakLoot _outitem))
  (for _index (range 1 (Math|Random|RandomIntegerinRange 1 3))
    (Utilities|Map|Add (LocalVariables|GetGeneratedLoots) _item (Math|Random|RandomIntegerinRange _minquantity _maxquantity)))
  (return (LocalVariables|GetGeneratedLoots)))

(fn ToGameplayEffectSpecHandle
  (params (Descriptor :type Gameplay%20Effect%20Descriptor%20Structure))
  (bind _returnvalue (Ability|GameplayEffect|AssignTagSetbyCallerMagnitude (GameplayEffects|MakeOutgoingSpec :self (Ability|GetAbilitySystemComponent 0) :GameplayEffectClass (.gameplayeffecttype Descriptor) :Level 1.0) (.datatag Descriptor) (Math|Conversions|ToFloat(Integer) (.magnitude Descriptor))))
  (bind _returnvalue_2 (Ability|GameplayEffect|AddAssetTag _returnvalue (.assettag Descriptor)))
  (return _returnvalue_2 (.bisreflexive Descriptor)))