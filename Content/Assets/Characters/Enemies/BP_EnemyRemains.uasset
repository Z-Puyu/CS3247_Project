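; BP_EnemyRemains is an interactable loot container representing what an enemy leaves behind.
; On BeginPlay it applies its mesh to the child static mesh actor and prints a debug message.
; It extends parent range events to open and close the player's loot container display with its Loots map.
; Interact gives every entry to the PlayerState, playing a scrapping sound per item, then destroys the actor.
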(event EventBeginPlay
  (bind _asstatic_mesh_actor (Utilities|Casting|CastToStaticMeshActor (Variables|/Script/Engine.ChildActorComponent|GetChildActor (Variables|Default|GetInteractableActor))))
  (Components|StaticMesh|SetStaticMesh (Variables|/Script/Engine.StaticMeshActor|GetStaticMeshComponent _asstatic_mesh_actor) (Variables|Default|GetMesh))
  (Development|PrintString "Enemy remains spawned!"))

(event EventOnPlayerinRange
  (params (Player :type Player%20Character%20Object%20Reference))
  (|CallParentFunction Player)
  (Default|CallOnOpenLootContainer (Variables|Default|GetPlayerInRange) (Variables|Default|GetLoots)))

(event EventOnPlayerOutOfRange
  (params (Player :type Player%20Character%20Object%20Reference))
  (Default|CallOnCloseLootContainer (Variables|Default|GetPlayerInRange))
  (|CallParentFunction Player))

(event Input|ActionEvents|InputActionInteract
  (params (Key :type Key%20Structure :default "None"))
  (bind _loots (Variables|Default|GetLoots))
  (:Pressed
    (bind _playerstate (Default|GetPlayerState (Variables|Default|GetPlayerInRange)))
    (bind _keys (Utilities|Map|Keys _loots))
    (for _array_element _keys
      (Default|EventonCollectItems _playerstate _array_element (.Value (Utilities|Map|Find _loots _array_element)))
      (Audio|PlaySoundatLocation "/Game/Audio/SFX/Player/Scrapping_Cue.Scrapping_Cue" (Transformation|GetActorLocation) "0, 0, 0" 1.0 1.0 0.0 0 0 0 0))
    (Actor|DestroyActor)))

(fn ConstructionScript)