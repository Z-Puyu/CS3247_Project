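; Player character Blueprint for a game with turn-based card combat, built on Gameplay Ability System attributes.
; Combat events toggle movement, input mode and cursor, relay turn changes, refill mana via a GameplayEffect, and check card costs against an attribute.
; Attribute changes drive low-health panting audio and the dead flag, while death plays a sound.
; OnLoad restores transform and attributes, but BeginPlay's save read and GetSaveData's body are disconnected.
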(event Custom|BattleStart
  (Pawn|Components|CharacterMovement|SetMovementMode (Variables|Character|GetCharacterMovement) "MOVE_None" 0)
  (Default|CallOnHealthUpdate)
  (Variables|Default|SetInBattle true))

(event Custom|Event%20On%20Player%20Death
  (Audio|PlaySoundatLocation "/Game/Audio/SFX/Combat/Player_Dies_Cue.Player_Dies_Cue" (Transformation|GetActorLocation) "0, 0, 0" 1.0 1.0 0.0 0 0 0 0))

(event Custom|Event%20On%20Check%20Health
  (params (HP :type Integer))
  (if (<= HP 0)
    (Variables|Default|SetIsDead true)
    (elif (<= HP (/ (.ReturnValue (Class|AbilitySystemComponent|GetGameplayAttributeValue (Variables|Default|GetAbilitySystemComponent) "(AttributeName=\"MaxHealth\",Attribute=/Script/CS3247_Project.BasicAttributeSet:MaxHealth,AttributeOwner=\"/Script/CoreUObject.Class'/Script/CS3247_Project.BasicAttributeSet'\")")) 3.0))
      (Audio|Components|Audio|Play (Variables|Default|GetPantingAudio) 0.0)
      (else
        (Audio|Components|Audio|FadeOut (Variables|Default|GetPantingAudio) 5.0 0.0 "Linear" :!class /Script/Engine.AudioComponent)))))

(event Custom|BattleEnd
  (Pawn|Components|CharacterMovement|SetMovementMode (Variables|Character|GetCharacterMovement) "MOVE_Walking" 0)
  (Variables|Default|SetInBattle false))

(event Custom|Event%20On%20Attribute%20Changed
  (params (Attribute :type Gameplay%20Attribute%20Structure) (OldValue :type Integer) (CurrentValue :type Integer))
  (if (== Attribute "(AttributeName=\"Health\",Attribute=/Script/CS3247_Project.BasicAttributeSet:Health,AttributeOwner=\"/Script/CoreUObject.Class'/Script/CS3247_Project.BasicAttributeSet'\")")
    (CallFunction|EventonCheckHealth CurrentValue)))

(event EventBeginPlay
  (bind _returnvalue (Game|GetPlayerController 0))
  (EventDispatchers|BindEventtoOnAttributeChanged (Variables|Default|GetAttributeSet) (delegate Custom|Event%20On%20Attribute%20Changed))
  (Input|SetInputModeGameOnly _returnvalue false)
  (Variables|/Script/Engine.PlayerController|SetbShowMouseCursor _returnvalue false)
  (Utilities|Casting|CastToBP_PlayerController _returnvalue)
  (Default|CallOnPlayerInitialised)
  (EventDispatchers|BindEventtoOnDeath (delegate Custom|Event%20On%20Player%20Death)))

(event Custom|Event%20On%20Load
  (params (SavedPlayerData :type S%20Player%20Save%20Data%20Structure))
  (bind (_transform _attributes _camerarotation) (Utilities|Struct|BreakS_PlayerSaveData SavedPlayerData))
  (Development|PrintString (Utilities|String|ToString(Transform) _transform))
  (Transformation|SetActorTransform _transform)
  (Class|BasicCharacter|LoadAttributes _attributes))

(event Custom|Event%20On%20Enter%20Combat
  (Components|Movement|StopMovementImmediately (Variables|Character|GetCharacterMovement))
  (Pawn|Components|CharacterMovement|SetMovementMode (Variables|Character|GetCharacterMovement) "MOVE_None" 0)
  (Development|PrintString "Combat started!")
  (Input|SetInputModeUIOnly (Game|GetPlayerController 0) 0 "DoNotLock" false)
  (Variables|Default|SetInBattle true)
  (Default|CallOnPlayerEnteredCombat))

(event Custom|Event%20On%20End%20Turn
  (Development|PrintString "Player turn ends")
  (Default|CallOnTurnEnded))

(event Custom|Event%20On%20Player%20Turn%20Start
  (Variables|/Script/Engine.PlayerController|SetbShowMouseCursor (Game|GetPlayerController 0) true)
  (GameplayEffects|ApplyGameplayEffectToSelf :self (Variables|Default|GetAbilitySystemComponent) :GameplayEffectClass "/Game/Assets/GameplayAbilities/GameplayEffects/GE_RefillMana.GE_RefillMana_C" :Level 1.0)
  (Development|PrintString "Player takes turn!")
  (Default|CallOnNewTurnStarted)
  (Development|PrintString (Utilities|String|ToString(Float) (.ReturnValue (Class|AbilitySystemComponent|GetGameplayAttributeValue (Variables|Default|GetAbilitySystemComponent) "(AttributeName=\"Health\",Attribute=/Script/CS3247_Project.BasicAttributeSet:Health,AttributeOwner=\"/Script/CoreUObject.Class'/Script/CS3247_Project.BasicAttributeSet'\")")))))

(event Custom|Event%20On%20Exit%20Combat
  (bind _returnvalue (Game|GetPlayerController 0))
  (Pawn|Components|CharacterMovement|SetMovementMode (Variables|Character|GetCharacterMovement) "MOVE_Walking" 0)
  (Variables|Default|SetInBattle false)
  (Input|SetInputModeGameOnly _returnvalue false)
  (Variables|/Script/Engine.PlayerController|SetbShowMouseCursor _returnvalue false)
  (Variables|Default|SetInBattle true)
  (Default|CallOnPlayerExitedCombat))

(fn ConstructionScript)

(fn PrintSpellsLR
  (params (RightSpell :type OneHandedSpells_Enum%20Enum :default "NewEnumerator0") (LeftSpell :type OneHandedSpells_Enum%20Enum :default "NewEnumerator0"))
  (Development|PrintString (Utilities|String|Append "R: " (Utilities|String|EnumtoString RightSpell)) true true "(R=0.000000,G=0.660000,B=1.000000,A=1.000000)" 3.0)
  (Development|PrintString (Utilities|String|Append "L: " (Utilities|String|EnumtoString LeftSpell)) true true "(R=0.000000,G=0.660000,B=1.000000,A=1.000000)" 3.0))

(fn SetTurnManager
  (params (manager :type BP%20Turn%20Manager%20Object%20Reference))
  (Variables|Default|SetTurnManager manager))

(fn OnPlayerTurn
  (Development|PrintString "My turn!")
  (return false))

(fn GetSaveData)

(fn CanPlayCard
  (params (Card :type Card%20Object%20Reference))
  (return (<= (.UseCost (Class|Card|GetCardData Card)) (.ReturnValue (Class|AbilitySystemComponent|GetGameplayAttributeValue (Ability|GetAbilitySystemComponent 0) "(AttributeName=\"Mana\",Attribute=/Script/CS3247_Project.PlayerAttributeSet:Mana,AttributeOwner=\"/Script/CoreUObject.Class'/Script/CS3247_Project.PlayerAttributeSet'\")")))))