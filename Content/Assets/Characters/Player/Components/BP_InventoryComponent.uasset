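; Player inventory component that adds and removes items and toggles the inventory screen.
; Pressing I adds the inventory widget to the viewport, or removes it when visible.
; Single-item events forward to the quantity-based add and remove events with a quantity of one.
; Those events call AddItem or RemoveItem, then broadcast OnInventoryChanged with the item and returned quantity.
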(event Input|KeyboardEvents|I
  (params (Key :type Key%20Structure :default "None"))
  (bind _inventorywidget (Variables|Default|GetinventoryWidget))
  (:Pressed
    (if (Widget|IsVisible (Variables|Default|GetinventoryWidget))
      (Widget|RemovefromParent _inventorywidget)
      (else
        (UserInterface|Viewport|AddtoViewport _inventorywidget 0)))))

(event Custom|Event%20On%20Remove%20Item
  (params (GameItem :type Game%20Item%20Object%20Reference) (Qty :type Integer))
  (bind _returnvalue (Class|InventoryComponent|RemoveItem GameItem Qty))
  (Default|CallOnInventoryChanged GameItem _returnvalue))

(event Custom|Event%20On%20Add%20Single%20Item
  (params (Item :type Game%20Item%20Object%20Reference))
  (CallFunction|EventonAddItem Item 1))

(event Custom|Event%20On%20Add%20Item
  (params (GameItem :type Game%20Item%20Object%20Reference) (Qty :type Integer))
  (bind _returnvalue (Class|InventoryComponent|AddItem GameItem Qty))
  (Default|CallOnInventoryChanged GameItem _returnvalue))

(event Custom|Event%20On%20Remove%20Single%20Item
  (params (Item :type Game%20Item%20Object%20Reference))
  (CallFunction|EventonRemoveItem Item 1))