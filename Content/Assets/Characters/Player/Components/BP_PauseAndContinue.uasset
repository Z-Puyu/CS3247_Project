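; BP_PauseAndContinue is a player component that pauses and resumes the game, keeping the InPause flag on BP_PlayerCharacter in sync.
; GamePause sets game-only input mode, creates WBP_PauseMenu, stores it in PausePanel, shows the cursor and pauses the game.
; GameContinue removes that stored widget, hides the cursor, unpauses and turns off ignoring of look input.
; Both functions do nothing unless the owner is BP_PlayerCharacter.
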(event EventBeginPlay)

(event EventTick
  (params (DeltaSeconds :type Float%20%28single-precision%29)))

(fn GamePause
  (bind _returnvalue (Game|GetPlayerController 0))
  (bind _asbp_player_character (Utilities|Casting|CastToBP_PlayerCharacter (Components|GetOwner)))
  (Variables|/Game/Assets/Characters/Player/BP_PlayerCharacter.BP_PlayerCharacter_C|SetInPause _asbp_player_character true)
  (Input|SetInputModeGameOnly _returnvalue false)
  (bind _returnvalue_2 (UserInterface|CreateWidget "/Game/UI/Menu/WBP_PauseMenu.WBP_PauseMenu_C"))
  (Variables|Default|SetPausePanel _returnvalue_2)
  (UserInterface|Viewport|AddtoViewport _returnvalue_2 0)
  (Variables|/Script/Engine.PlayerController|SetbShowMouseCursor _returnvalue true)
  (Game|SetGamePaused true))

(fn GameContinue
  (bind _returnvalue (Game|GetPlayerController 0))
  (bind _asbp_player_character (Utilities|Casting|CastToBP_PlayerCharacter (Components|GetOwner)))
  (Variables|/Game/Assets/Characters/Player/BP_PlayerCharacter.BP_PlayerCharacter_C|SetInPause _asbp_player_character false)
  (Widget|RemovefromParent (Variables|Default|GetPausePanel))
  (Variables|/Script/Engine.PlayerController|SetbShowMouseCursor _returnvalue false)
  (Game|SetGamePaused false)
  (Input|SetIgnoreLookInput _returnvalue false))