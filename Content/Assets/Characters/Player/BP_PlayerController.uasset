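; Player controller for a card-based dungeon game, linking the player to combat, card play and interaction events.
; Played cards go to the card executor component, and a handler is bound to the card crafter on BeginPlay.
; Combat events toggle the cursor, switch between UI and game input on start and end, and fire dispatchers.
; Interaction zone and enchanting station events are relayed through dispatchers.
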(event Custom|Event%20On%20Play%20Card
  (params (TargetCharacter :type Basic%20Character%20Object%20Reference) (Card :type Card%20Object%20Reference))
  (Default|EventonExecuteCard (Variables|Default|GetCardExecutorComponent) Card))

(event EventBeginPlay
  (bind _asbp_dungeon_slayer_player_state (Utilities|Casting|CastToBP_DungeonSlayerPlayerState (Variables|GetPlayerState)))
  (EventDispatchers|BindEventtoOnCardCrafted (Variables|Default|GetCardCrafterComponent) (EventDispatchers|CreateEvent (Variables|/Game/Assets/Characters/Player/BP_DungeonSlayerPlayerState.BP_DungeonSlayerPlayerState_C|GetPlayerDeck _asbp_dungeon_slayer_player_state) :!event AddCard)))

(event Custom|Event%20On%20Combat%20Start
  (Default|CallOnCombatStarted)
  (Development|PrintString "Combat started!")
  (Input|SetInputModeUIOnly self 0 "DoNotLock" false))

(event Custom|Event%20On%20End%20Turn
  (Development|PrintString "Player turn ends")
  (Variables|Default|SetbShowMouseCursor false)
  (Default|CallOnPlayerTurnEnded))

(event Custom|Event%20On%20Player%20Turn%20Start
  (Variables|Default|SetbShowMouseCursor true)
  (Development|PrintString "Player takes turn!")
  (Default|CallOnPlayerTurnStarted))

(event Custom|Event%20On%20Combat%20End
  (params (Winner :type E_CombatWinner%20Enum :default "NewEnumerator0"))
  (switch Utilities|FlowControl|Switch|SwitchonE_CombatWinner Winner
    (:NewEnumerator0
      (Variables|Default|SetbShowMouseCursor false)
      (Input|SetInputModeGameOnly self false)
      (Default|CallOnCombatEnded true))
    (:NewEnumerator1
      (Variables|Default|SetbShowMouseCursor true)
      (Input|SetInputModeUIOnly self 0 "DoNotLock" false)
      (Default|CallOnCombatEnded false))))

(event Custom|Event%20On%20Enter%20Interaction%20Zone
  (params (Prompt%20Text :type Text))
  (Default|CallOninRangeforInteraction Prompt%20Text))

(event Custom|Event%20On%20Leave%20Interaction%20Zone
  (Default|CallOnLeaveInteractionZone))

(event Custom|Event%20On%20Use%20Enchanting%20Station
  (Default|CallOnUseEnchantingStation))

(fn ConstructionScript)

(fn GetPlayerState
  (bind _asbp_dungeon_slayer_player_state (Utilities|Casting|CastToBP_DungeonSlayerPlayerState (Variables|GetPlayerState)))
  (return _asbp_dungeon_slayer_player_state))