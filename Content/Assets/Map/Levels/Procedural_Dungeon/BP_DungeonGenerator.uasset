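; Procedural dungeon generator that grows a level from a start room by spawning random rooms at random open exits.
; After a short delay, each room's overlap boxes are tested; colliding rooms are destroyed and retried, while accepted ones add exits and floor points.
; Once the room count is met, it walls unused exits and recursively places encounter zones.
; A watchdog timer reloads the test level if generation runs too long.
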(event Custom|SpawnStartRoom
  ;[0.1015 0.15 0.03687 0.5] Spawn Start Room
  (bind _returnvalue (Game|SpawnActorfromClass "/Game/Assets/Map/Levels/Procedural_Dungeon/BP_FirstRoom.BP_FirstRoom_C" (Transformation|GetWorldTransform (Variables|Default|GetDefaultSceneRoot)) "AlwaysSpawn" "MultiplyWithRoot" 0 0))
  (Utilities|Array|AppendArray (Variables|Default|GetexitsList) (Components|GetChildrenComponents (Variables|/Game/Assets/Map/Levels/Procedural_Dungeon/BP_MasterRoom.BP_MasterRoom_C|GetExitFolder _returnvalue) false)))

(event Custom|Add%20Overlapping%20Rooms%20To%20List
  ;[0.006128 0.15 0 0.5] Check Overlapping Room
  (for _array_element (Components|GetChildrenComponents (Variables|/Game/Assets/Map/Levels/Procedural_Dungeon/BP_MasterRoom.BP_MasterRoom_C|GetOverlapFolder (Variables|Default|GetlatestRoom)) false)
    (bind _asbox_collision (Utilities|Casting|CastToBoxComponent _array_element))
    (Variables|Default|SetOverlapped%20List (Class|PrimitiveComponent|GetOverlappingComponents _asbox_collision))))

(event Custom|SpawnNextRoom
  ;[0.04319 0.15 0.02494 0.5] Spawn Next Room
  (bind _output_get (Variables|Default|SetselectedExit (.OutItem (Utilities|Array|Random (Variables|Default|GetexitsList)))))
  (bind _returnvalue (Game|SpawnActorfromClass (.OutItem (Utilities|Array|Random (Variables|Default|GetroomList))) (Transformation|GetWorldTransform _output_get) "Undefined" "MultiplyWithRoot" 0 0))
  (bind _asbp_master_room (Utilities|Casting|CastToBP_MasterRoom _returnvalue))
  (Variables|Default|SetlatestRoom _asbp_master_room)
  (Utilities|FlowControl|Delay 0.01)
  (CallFunction|FixOverlap))

(event Custom|Fix%20Overlap
  (bind _overlapped_list (Variables|Default|GetOverlapped%20List))
  ;[0.006128 0.15 0 0.5] Fix Overlap
  (CallFunction|AddOverlappingRoomstoList)
  (if (Utilities|Array|IsNotEmpty (Variables|Default|GetOverlapped%20List))
    (Utilities|Array|Clear _overlapped_list)
    (Actor|DestroyActor (Variables|Default|GetlatestRoom))
    (CallFunction|SpawnNextRoom)
    (else
      (Utilities|Array|Clear _overlapped_list)
      (Variables|Default|SetnumOfRooms (- (Variables|Default|GetnumOfRooms) 1))
      (Utilities|Array|RemoveItem (Variables|Default|GetexitsList) (Variables|Default|GetselectedExit))
      (Utilities|Array|AppendArray (Variables|Default|GetexitsList) (Components|GetChildrenComponents (Variables|/Game/Assets/Map/Levels/Procedural_Dungeon/BP_MasterRoom.BP_MasterRoom_C|GetExitFolder (Variables|Default|GetlatestRoom)) false))
      (Utilities|Array|AppendArray (Variables|Default|GetFloor%20Spawn%20List) (Components|GetChildrenComponents (Variables|/Game/Assets/Map/Levels/Procedural_Dungeon/BP_MasterRoom.BP_MasterRoom_C|GetFloorSpawnPointFolder (Variables|Default|GetlatestRoom)) false))
      (if (> (Variables|Default|GetnumOfRooms) 0)
        (CallFunction|SpawnNextRoom)
        (else
          (CallFunction|CloseUnusedExits)
          (CallFunction|SpawnEnemiesatLocation)
          (Variables|Default|SetisComplete true)
          (Utilities|Time|ClearandInvalidateTimerbyHandle (Variables|Default|GetTimer%20Handle))
          (Development|PrintString "Hello"))))))

(event Custom|Close%20Unused%20Exits
  ;[0 0.15 0.009936 0.5] Closed Unused Exits
  (for _array_element (Variables|Default|GetexitsList)
    (Game|SpawnActorfromClass "/Game/Assets/Map/Levels/Procedural_Dungeon/BP_Wall.BP_Wall_C" (Transformation|GetWorldTransform _array_element) "Undefined" "MultiplyWithRoot" 0 0)))

(event Custom|Start%20Dungeon%20Timer
  ;[0 0.15 0.02745 0.5] Timer Handler
  (bind _returnvalue (Utilities|Time|SetTimerbyEvent (delegate Custom|Check%20Completion) 1.0 true))
  (Variables|Default|SetTimer%20Handle _returnvalue))

(event Custom|Check%20Completion
  ;[0 0.15 0.02745 0.5] Timer Handler
  (if (>= (Utilities|Time|GetGameTimeinSeconds) 15.0)
    (Game|OpenLevel(byName) "LV_ProceduralDungeonTest")))

(event Custom|Spawn%20Enemies%20at%20Location
  ;[0 0.15 0.006359 0.5] Spawn Enemis at Random Location
  (if (> (Variables|Default|GetnumOfEnemies) 0)
    (Variables|Default|SetnumOfEnemies (- (Variables|Default|GetnumOfEnemies) 1))
    (Variables|Default|SetSelectedFloorPoint (.OutItem (Utilities|Array|Random (Variables|Default|GetFloor%20Spawn%20List))))
    (Game|SpawnActorfromClass "/Game/Assets/Combat/BP_EncounterZone_Old.BP_EncounterZone_Old_C" (Math|Transform|MakeTransform (Transformation|GetWorldLocation (Variables|Default|GetSelectedFloorPoint)) "0, 0, 0" "3.000000,3.000000,3.000000") "Undefined" "MultiplyWithRoot" 0 0)
    (Utilities|Array|RemoveItem (Variables|Default|GetFloor%20Spawn%20List) (Variables|Default|GetSelectedFloorPoint))
    (CallFunction|SpawnEnemiesatLocation)))

(event EventBeginPlay
  (CallFunction|SpawnStartRoom)
  (CallFunction|StartDungeonTimer)
  (CallFunction|SpawnNextRoom))

(event Collision|EventActorBeginOverlap
  (params (OtherActor :type Actor%20Object%20Reference)))

(event EventTick
  (params (DeltaSeconds :type Float%20%28single-precision%29)))

(fn ConstructionScript)