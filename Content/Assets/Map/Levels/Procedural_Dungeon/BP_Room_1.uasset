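; BP_Room_1 is a procedural dungeon room that has a random chance to hold an enchanting station and a treasure chest.
; On BeginPlay, after the parent logic, a coin flip gathers the child spawn points, places the station facing an arrow component, removes a random point, then places the chest.
; Each random pick is a separate call, so the removed point may differ from the station's and both actors can share a location.
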(event EventBeginPlay
  (|CallParentFunction)
  (if (Math|Random|RandomBool)
    (bind _output_get (Variables|Default|SetenchantingTableSpawnPointArray (Components|GetChildrenComponents (Variables|Default|GetEnchantingTableSpawnPointFolder) false)))
    (Game|SpawnActorfromClass "/Game/Assets/MapInteractables/BP_EnchantingStationInteractable.BP_EnchantingStationInteractable_C" (Math|Transform|MakeTransform (Transformation|GetWorldLocation (.OutItem (Utilities|Array|Random _output_get))) (Math|Rotator|FindLookatRotation (Transformation|GetWorldLocation (.OutItem (Utilities|Array|Random _output_get))) (Transformation|GetWorldLocation (Variables|Default|GetArrow))) "1.000000,1.000000,1.000000") "Undefined" "MultiplyWithRoot" 0 0)
    (Utilities|Array|RemoveItem (Variables|Default|GetenchantingTableSpawnPointArray) (.OutItem (Utilities|Array|Random _output_get)))
    (Game|SpawnActorfromClass "/Game/Assets/MapInteractables/BP_TreasureChestInteractable.BP_TreasureChestInteractable_C" (Math|Transform|MakeTransform (Transformation|GetWorldLocation (.OutItem (Utilities|Array|Random (Variables|Default|GetenchantingTableSpawnPointArray)))) "0, 0, 0" "1.000000,1.000000,1.000000") "Undefined" "MultiplyWithRoot" 0 0 0)))

(event Collision|EventActorBeginOverlap
  (params (OtherActor :type Actor%20Object%20Reference))
  (|CallParentFunction OtherActor) ; This node is disabled and will not be called.\nDrag off pins to build functionality.
)

(event EventTick
  (params (DeltaSeconds :type Float%20%28single-precision%29))
  (|CallParentFunction DeltaSeconds) ; This node is disabled and will not be called.\nDrag off pins to build functionality.
)

(fn ConstructionScript
  (|CallParentFunction))