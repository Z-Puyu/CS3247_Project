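; BP_ProceduralMap generates a random dungeon on BeginPlay, then triggers map object and enemy spawning in its rooms.
; From a random start room, it recursively attaches room templates to open exits until DungeonSize hits zero, then places a portal room.
; Overlapping rooms are destroyed and their exits later walled, while remaining open exits get dead ends.
; DangerLevel sets the share of shuffled rooms receiving enemies; older encounter-zone and timer events are never called here.
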(event Custom|Event%20On%20Spawn%20Start%20Room
  ;[0.15 0.15 0.15 0.5] Room placement logic
  ;;[0.15 0.15 0.15 0.5] Create the starting room
  (bind _returnvalue (Game|SpawnActorfromClass (.OutItem (Utilities|Array|Random (Variables|Generator|GetStartingRoomTemplates))) (Transformation|GetWorldTransform (Variables|Default|GetDefaultSceneRoot)) "AlwaysSpawn" "MultiplyWithRoot" 0 0))
  (Utilities|Array|RemoveItem (Variables|Generator|GetOpenEnds) (Variables|Generator|GetCurrentExit))
  (bind _exits (Default|FetchAllExits _returnvalue))
  (Utilities|Array|AppendArray (Variables|Generator|GetOpenEnds) _exits))

(event Custom|Event%20On%20Spawn%20Enemies
  (Utilities|Array|Shuffle (Variables|Generator|GetRooms))
  (for _index (range 0 (- (Math|Float|Round (* (Utilities|Array|Length (Variables|Generator|GetRooms)) (Variables|Generator|GetDangerLevel))) 1))
    (Default|EventonSpawnEnemies (Utilities|Array|Get(acopy) (Variables|Generator|GetRooms) _index))))

(event Custom|Event%20On%20Fix%20Overlapping%20Room
  (params (Room :type BP%20Room%20Object%20Reference))
  ;[0.15 0.15 0.15 0.5] Room placement logic
  ;;[0.15 0.15 0.15 0.5] Fix overlap
  (Actor|DestroyActor Room)
  (Utilities|Array|Add (Variables|Generator|GetUnusableExits) (Variables|Generator|GetCurrentExit))
  (Utilities|Array|RemoveItem (Variables|Generator|GetOpenEnds) (Variables|Generator|GetCurrentExit))
  (Variables|Generator|SetCurrentExit 0))

(event Custom|Event%20On%20Spawn%20Dead%20End
  ;[0.15 0.15 0.15 0.5] Room placement logic
  ;;[0.15 0.15 0.15 0.5] Spawn Dead End Room
  (bind _output_get (Variables|Generator|SetCurrentExit (.OutItem (Utilities|Array|Random (Variables|Generator|GetOpenEnds)))))
  (bind _returnvalue (Game|SpawnActorfromClass "/Game/Assets/Map/ProceduralGeneration/Rooms/BP_RoomDeadEnd.BP_RoomDeadEnd_C" (Transformation|GetWorldTransform _output_get) "Undefined" "MultiplyWithRoot" 0 0))
  (bind _biscolliding (Default|IsColliding _returnvalue))
  (if _biscolliding
    (CallFunction|EventonFixOverlappingRoom _returnvalue)
    (else
      (CallFunction|EventonAddNewRoom _returnvalue))))

(event Custom|Event%20On%20Spawn%20Map%20Objects
  (for _array_element (Variables|Generator|GetRooms)
    (Default|EventonSpawnMapObjects _array_element)))

(event Custom|Event%20On%20Spawn%20Next%20Room
  ;[0.15 0.15 0.15 0.5] Room placement logic
  ;;[0.15 0.15 0.15 0.5] Spawn a common room
  (bind _output_get (Variables|Generator|SetCurrentExit (.OutItem (Utilities|Array|Random (Variables|Generator|GetOpenEnds)))))
  (bind _returnvalue (Game|SpawnActorfromClass (.OutItem (Utilities|Array|Random (Variables|Generator|GetRoomTemplates))) (Transformation|GetWorldTransform _output_get) "Undefined" "MultiplyWithRoot" 0 0))
  (bind _biscolliding (Default|IsColliding _returnvalue))
  (if _biscolliding
    (CallFunction|EventonFixOverlappingRoom _returnvalue)
    (CallFunction|EventonSpawnNextRoom :!label _label)
    (else
      (CallFunction|EventonAddNewRoom _returnvalue)
      (if (== (Variables|Generator|GetDungeonSize) 0)
        (CallFunction|EventonSpawnLastRoom)
        (else
          (goto _label))))))

(event Custom|Close%20Unused%20Exits
  ;[0.15 0.15 0.15 0.5] Room placement logic
  ;;[0.15 0.15 0.15 0.5] Close Unused Open Ends
  (while (Utilities|Array|IsNotEmpty (Variables|Generator|GetOpenEnds))
    (CallFunction|EventonSpawnDeadEnd))
  (for _array_element (Variables|Generator|GetUnusableExits)
    (Game|SpawnActorfromClass "/Game/Assets/Map/Levels/Procedural_Dungeon/BP_Wall.BP_Wall_C" (Transformation|GetWorldTransform _array_element) "Undefined" "MultiplyWithRoot" 0 0)))

(event Custom|Start%20Dungeon%20Timer
  ;[0 0.15 0.02745 0.5] Timer Handler
  (bind _returnvalue (Utilities|Time|SetTimerbyEvent (delegate Custom|Check%20Completion) 1.0 true))
  (Variables|Default|SetTimer%20Handle _returnvalue))

(event Custom|Check%20Completion
  ;[0 0.15 0.02745 0.5] Timer Handler
  (if (>= (Utilities|Time|GetGameTimeinSeconds) 15.0)
    (Game|OpenLevel(byName) "LV_ProceduralDungeonTest")))

(event Custom|Event%20On%20Add%20New%20Room
  (params (Room :type BP%20Room%20Object%20Reference))
  ;[0.15 0.15 0.15 0.5] Register a new room
  (Utilities|Array|RemoveItem (Variables|Generator|GetOpenEnds) (Variables|Generator|GetCurrentExit))
  (Utilities|Array|Add (Variables|Generator|GetRooms) Room)
  (bind _exits (Default|FetchAllExits Room))
  (Utilities|Array|AppendArray (Variables|Generator|GetOpenEnds) _exits)
  (bind _result (Math|Integer|DecrementInt (Variables|Generator|GetDungeonSize))))

(event Custom|Spawn%20Enemies%20at%20Location
  ;[0 0.15 0.006359 0.5] Spawn Enemis at Random Location
  (if (> (Variables|Generator|GetDangerLevel) 0)
    (Variables|Generator|SetDangerLevel (- (Variables|Generator|GetDangerLevel) 1))
    (Variables|Default|SetSelectedFloorPoint (.OutItem (Utilities|Array|Random (Variables|Default|GetFloor%20Spawn%20List))))
    (Game|SpawnActorfromClass "/Game/Assets/Combat/BP_EncounterZone_Old.BP_EncounterZone_Old_C" (Math|Transform|MakeTransform (Transformation|GetWorldLocation (Variables|Default|GetSelectedFloorPoint)) "0, 0, 0" "3.000000,3.000000,3.000000") "Undefined" "MultiplyWithRoot" 0 0)
    (Utilities|Array|RemoveItem (Variables|Default|GetFloor%20Spawn%20List) (Variables|Default|GetSelectedFloorPoint))
    (CallFunction|SpawnEnemiesatLocation)))

(event Custom|Event%20On%20Spawn%20Last%20Room
  ;[0.15 0.15 0.15 0.5] Room placement logic
  ;;[0.15 0.15 0.15 0.5] Spawn Portak Room
  (bind _output_get (Variables|Generator|SetCurrentExit (.OutItem (Utilities|Array|Random (Variables|Generator|GetOpenEnds)))))
  (bind _returnvalue (Game|SpawnActorfromClass "/Game/Assets/Map/ProceduralGeneration/Rooms/BP_PortalRoom.BP_PortalRoom_C" (Transformation|GetWorldTransform _output_get) "Undefined" "MultiplyWithRoot" 0 0))
  (bind _biscolliding (Default|IsColliding _returnvalue))
  (if _biscolliding
    (CallFunction|EventonFixOverlappingRoom _returnvalue)
    (CallFunction|EventonSpawnLastRoom)
    (else
      (CallFunction|EventonAddNewRoom _returnvalue)
      (CallFunction|CloseUnusedExits))))

(event EventBeginPlay
  (CallFunction|EventonSpawnStartRoom)
  (CallFunction|EventonSpawnNextRoom)
  (CallFunction|EventonSpawnMapObjects)
  (CallFunction|EventonSpawnEnemies))

(fn ConstructionScript)