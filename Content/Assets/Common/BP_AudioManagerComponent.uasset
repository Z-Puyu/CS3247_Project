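; Audio manager component that runs background music, switching between an ambient track and a combat track.
; On BeginPlay it adds an audio component per track to its owner, async loads both, and spawns ambient effects as 2D sound.
; The ambient track replays after random pauses unless combat music is playing.
; Combat start and stop events fade between them, with ambient playback retried after a short delay when combat ends.
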(event Custom|Event%20On%20Track%20Finished
  (Utilities|Time|SetTimerbyEvent (delegate Custom|Event%20On%20Play%20Next%20Track) (Math|Random|RandomFloatinRange (Variables|BackgroundTrack|GetMinDelayBetweenTracks) (Variables|BackgroundTrack|GetMaxDelayBetweenTracks))))

(event Custom|Event%20On%20Play%20Combat%20Music
  (if (Audio|Components|Audio|IsPlaying (Variables|Default|GetAmbientAudio))
    (Audio|Components|Audio|FadeOut (Variables|Default|GetAmbientAudio) 0.5 0.0 "Linear" :!class /Script/Engine.AudioComponent))
  (Audio|Components|Audio|FadeIn (Variables|Default|GetCombatAudio) 5.0 1.0 0.0 "Linear" :!class /Script/Engine.AudioComponent))

(event Custom|Event%20On%20Stop%20Combat%20Music
  (Audio|Components|Audio|FadeOut (Variables|Default|GetCombatAudio) 1.0 0.0 "Linear" :!class /Script/Engine.AudioComponent)
  (Utilities|FlowControl|Delay 5.0)
  (CallFunction|EventonPlayNextTrack))

(event Custom|Event%20On%20Play%20Next%20Track
  (if (not (Audio|Components|Audio|IsPlaying (Variables|Default|GetCombatAudio)))
    (Audio|Components|Audio|Play (Variables|Default|GetAmbientAudio) 0.0)
    (EventDispatchers|BindEventtoOnAudioFinished (Variables|Default|GetAmbientAudio) (delegate Custom|Event%20On%20Track%20Finished))))

(event EventBeginPlay
  (bind _ambienttrack (Variables|BackgroundTrack|GetAmbientTrack))
  (bind _combattrack (Variables|Default|GetCombatTrack))
  (bind _ambientsoundeffects (Variables|Default|GetAmbientSoundEffects))
  (bind _returnvalue (Game|AddComponentbyClass (Components|GetOwner) "/Script/Engine.AudioComponent" false))
  (bind _output_get (Variables|Default|SetAmbientAudio _returnvalue))
  (Utilities|AsyncLoadAsset _ambienttrack
    (:then
      (bind _returnvalue_2 (Game|AddComponentbyClass (Components|GetOwner) "/Script/Engine.AudioComponent" false))
      (Variables|Default|SetCombatAudio _returnvalue_2)
      (Utilities|AsyncLoadAsset _combattrack
        (:then
          (Utilities|AsyncLoadAsset _ambientsoundeffects
            (:Completed
              (Audio|SpawnSound2D (Utilities|ResolveSoftReference _ambientsoundeffects) 1.0 1.0 0.0 0 true))))
        (:Completed
          (Audio|Components|Audio|SetSound (Variables|Default|GetCombatAudio) (Utilities|ResolveSoftReference _combattrack)))))
    (:Completed
      (Audio|Components|Audio|SetSound _output_get (Utilities|ResolveSoftReference _ambienttrack))
      (CallFunction|EventonPlayNextTrack))))