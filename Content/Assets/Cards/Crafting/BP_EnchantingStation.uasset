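; Enchanting station actor for card crafting that links its activation state to its candle child actors.
; On BeginPlay it loops through all child actors, casts them to BP_EnchantingStationCandle and binds OnActivated and OnDeactivated events for the candles.
; Its OnActivate and OnDeactivate events fire those dispatchers, so the candles follow the station through event dispatchers.
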(event Custom|Event%20On%20Activate
  (Default|CallOnActivated))

(event Custom|Event%20On%20Deactivate
  (Default|CallOnDeactivated))

(event EventBeginPlay
  (for _array_element (Actor|GetAllChildActors true)
    (bind _asbp_enchanting_station_candle (Utilities|Casting|CastToBP_EnchantingStationCandle _array_element))
    (EventDispatchers|BindEventtoOnActivated (EventDispatchers|CreateEvent _asbp_enchanting_station_candle :!event EventonLit))
    (EventDispatchers|BindEventtoOnDeactivated (EventDispatchers|CreateEvent _asbp_enchanting_station_candle :!event EventonPutOff))))

(fn ConstructionScript)