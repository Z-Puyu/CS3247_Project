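; BP_Recipe is a crafting recipe object built from a CardRecipe and the player's deck.
; CardNodeToRecipe converts the recipe's edge list into BP_IngredientNode objects, each linking a From and To ingredient, and collects them in IngredientList.
; It then forges the Card from the deck, prints a message if that card is invalid, and returns itself.
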(fn CardNodetoRecipe
  (params (CardRecipe :type Card%20Recipe%20Object%20Reference) (PlayerDeck :type BP%20Player%20Deck%20Component%20Object%20Reference))
  (Utilities|FlowControl|Sequence
    (:then_0
      (bind _returnvalue (Class|CardRecipe|ToEdgeList CardRecipe))
      (if (> (Utilities|Array|Length _returnvalue) 0)
        (for _array_element _returnvalue
          (bind _returnvalue_2 (Game|ConstructObjectfromClass "/Game/Assets/Cards/Crafting/Recipe/BP_IngredientNode.BP_IngredientNode_C" (.Ingredient (Utilities|Struct|BreakIngredientKey (.From (Utilities|Struct|BreakRecipeEdge _array_element)))) (.Ingredient (Utilities|Struct|BreakIngredientKey (.To (Utilities|Struct|BreakRecipeEdge _array_element))))))
          (Utilities|Array|Add (Variables|Default|GetIngredientList) _returnvalue_2))))
    (:then_1
      (bind _output_get (Variables|Default|SetCard (Class|CardRecipe|Forge CardRecipe PlayerDeck)))
      (Utilities|IsValid _output_get
        (:Is%20Valid
          _)
        (:Is%20Not%20Valid
          (Development|PrintText 0 "invalid card data!")))
      (return self))))