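; BP_PlayerDeckComponent is a component that holds the player's card deck and exposes it for saving and loading.
; GetSaveData returns the Deck array, and OnLoad rebuilds it from saved data.
; BeginPlay separately fills InitialCards by forging each entry in TestRecipes, then prints the count.
; The hookup to a CardCrafter's card-crafted event is unfinished: both functions are empty, with their binding nodes disconnected.
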(event Custom|Event%20On%20Load
  (params (SaveData :type Array%20of%20Card%20Object%20References))
  (Utilities|Array|Clear (Variables|Default|GetDeck))
  (for _array_element SaveData
    (Utilities|Array|Add (Variables|Default|GetDeck) _array_element)))

(event EventBeginPlay
  (Utilities|Array|Clear (Variables|Default|GetInitialCards))
  (for _array_element (Variables|Default|GetTestRecipes)
    (Utilities|Array|Add (Variables|Default|GetInitialCards) (Class|CardRecipe|Forge _array_element self)))
  (Development|PrintText (Utilities|Text|FormatText (Utilities|Text|MakeLiteralText "Started with {0} cards") (Utilities|Array|Length (Variables|Default|GetInitialCards)))))

(fn ConnectEvents
  (params (CardCrafter :type BP%20Card%20Crafter%20Component%201%20Object%20Reference)))

(fn AddCardonNewCardCrafted
  (params (Card%20Crafter :type BP%20Card%20Crafter%20Component%201%20Object%20Reference)))

(fn GetSaveData
  (return (Variables|Default|GetDeck)))