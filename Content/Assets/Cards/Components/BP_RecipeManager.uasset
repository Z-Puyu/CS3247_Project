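; Component on the player controller that keeps a list of card recipes made with the card crafter.
; On BeginPlay it casts its owner to BP_PlayerController and caches that controller's CardCrafterComponent.
; Save appends the crafter's current recipe to ListOfRecipe, prints the new index and fires Saved with the recipe's card.
; Load is an empty stub, and nothing here writes the list to disk.
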(event Custom|Event%20Save
  (bind _current_recipe (Default|GetCurrentRecipe (Variables|Default|GetCardCrafterComponent)))
  (bind _returnvalue (Utilities|Array|Add (Variables|Default|GetListOfRecipe) _current_recipe))
  (Development|PrintString (Utilities|String|ToString(Integer) _returnvalue))
  (Default|CallSaved (Variables|/Game/Assets/Cards/Crafting/Recipe/BP_Recipe.BP_Recipe_C|GetCard _current_recipe)))

(event Custom|Event%20Load)

(event EventBeginPlay
  (bind _asbp_player_controller (Utilities|Casting|CastToBP_PlayerController (Components|GetOwner)))
  (bind _output_get (Variables|Default|SetOwningPlayer _asbp_player_controller))
  (Variables|Default|SetCardCrafterComponent (Variables|/Game/Assets/Characters/Player/BP_PlayerController.BP_PlayerController_C|GetCardCrafterComponent _output_get)))

(event EventTick
  (params (DeltaSeconds :type Float%20%28single-precision%29)))