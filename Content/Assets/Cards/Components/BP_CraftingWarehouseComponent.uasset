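; Component that serves as the crafting warehouse, tracking how many of each ingredient is available in a map.
; Add and use events update the map, with use consuming one unit and removing depleted entries, then broadcast the new quantity through dispatchers.
; LoadIngredients replays every stored entry through the add dispatcher so listeners receive the current stock.
; Requests for missing or insufficient ingredients print a warning.
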(event Custom|Event%20Load%20Ingredients
  (bind _availableingredients (Variables|Default|GetAvailableIngredients))
  (bind _keys (Utilities|Map|Keys _availableingredients))
  (for _array_element _keys
    (Default|CallOnAddIngredient _array_element (.Value (Utilities|Map|Find _availableingredients _array_element)))))

(event Custom|Event%20On%20Add%20Ingredient
  (params (Ingredient :type Card%20Ingredient%20Object%20Reference) (Qty :type Integer))
  (bind _currentqty (Warehouse|AddIngredient Ingredient Qty))
  (Default|CallOnAddIngredient Ingredient _currentqty))

(event Custom|Event%20On%20Use%20Ingredient
  (params (Ingredient :type Card%20Ingredient%20Object%20Reference))
  (bind _remainingqty (Warehouse|UseIngredient Ingredient))
  (Default|CallOnUseIngredient Ingredient _remainingqty))

(fn AddIngredient
  (params (Ingredient :type Card%20Ingredient%20Object%20Reference) (Qty :type Integer))
  (bind _availableingredients (Variables|Default|GetAvailableIngredients))
  (bind (_value _returnvalue) (Utilities|Map|Find _availableingredients Ingredient))
  (bind _output_get (LocalVariables|SetNewQty Qty))
  (if _returnvalue
    (LocalVariables|SetNewQty (+ _output_get _value)))
  (Utilities|Map|Add (Variables|Default|GetAvailableIngredients) Ingredient (LocalVariables|GetNewQty))
  (return (LocalVariables|GetNewQty)))

(fn UseIngredient
  (params (Ingredient :type Card%20Ingredient%20Object%20Reference))
  (bind _remainingqty (Warehouse|GetRemainingQuantity Ingredient 1))
  (bind _output_get (LocalVariables|SetRemaining _remainingqty))
  (if (> _output_get 0)
    (Utilities|Map|Add (Variables|Default|GetAvailableIngredients) Ingredient (LocalVariables|GetRemaining))
    (return (LocalVariables|GetRemaining))
    (else
      (Utilities|Map|Remove (Variables|Default|GetAvailableIngredients) Ingredient)
      (return 0))))

(fn GetRemainingQuantity
  (params (Ingredient :type Card%20Ingredient%20Object%20Reference) (QuantityUsed :type Integer))
  (bind _availableingredients (Variables|Default|GetAvailableIngredients))
  (bind (_value _returnvalue) (Utilities|Map|Find _availableingredients Ingredient))
  (LocalVariables|SetCurrentQty _value)
  (if _returnvalue
    (if (<= QuantityUsed (LocalVariables|GetCurrentQty))
      (return (- (LocalVariables|GetCurrentQty) QuantityUsed))
      (else
        (Development|PrintText (Utilities|Text|FormatText (Utilities|Text|MakeLiteralText "Want to use {0} copies of {1} but there are only {2}") QuantityUsed Ingredient (LocalVariables|GetCurrentQty)) true true "(R=1.000000,G=0.000000,B=0.000000,A=1.000000)")))
    (else
      (Development|PrintText (Utilities|Text|FormatText (Utilities|Text|MakeLiteralText "There is no {}") (Variables|/Script/CS3247_Project.CardIngredient|GetName Ingredient)) true true "(R=1.000000,G=0.000000,B=0.000000,A=1.000000)"))))