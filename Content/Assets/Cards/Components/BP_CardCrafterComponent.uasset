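; Player controller component that runs the card-crafting workbench, building a node-graph recipe and forging it into a new card.
; Ingredients are wrapped into nodes, which workbench events link, unlink or set as the recipe's root, printing results or errors.
; Crafting forges the recipe with the player state's deck, broadcasts the crafted card and starts a fresh session.
; GetCurrentRecipe converts the working graph into a BP_Recipe using that same deck.
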(event EventBeginPlay
  (bind _asbp_player_controller (Utilities|Casting|CastToBP_PlayerController (Components|GetOwner)))
  (Variables|Default|SetOwningPlayer _asbp_player_controller)
  (CallFunction|EventNewSession))

(event Custom|Event%20On%20Craft%20New%20Card
  ;[0.15 0.15 0.15 0.5] Craft a new card
  (Default|GetPlayerState (Variables|Default|GetOwningPlayer))
  (bind _playerstate (Default|GetPlayerState (Variables|Default|GetOwningPlayer)))
  (Default|CallOnCardCrafted (Class|CardRecipe|Forge (Variables|Default|GetCurrentRecipe) (Variables|/Game/Assets/Characters/Player/BP_DungeonSlayerPlayerState.BP_DungeonSlayerPlayerState_C|GetPlayerDeck _playerstate)))
  (Development|PrintString "New card crafted!")
  (CallFunction|EventNewSession))

(event Custom|Event%20NewSession
  ;[0.15 0.15 0.15 0.5] Start a new crafting session
  (bind _returnvalue (Game|ConstructObjectfromClass "/Script/CS3247_Project.CardRecipe"))
  (Variables|Default|SetCurrentRecipe _returnvalue))

(event Custom|Event%20On%20Set%20Root%20Node
  (params (Root :type Card%20Node%20Object%20Reference))
  (Variables|/Script/CS3247_Project.CardRecipe|SetSource (Variables|Default|GetCurrentRecipe) Root))

(event Custom|Event%20On%20Disconnect%20Nodes
  (params (ParentNode :type Card%20Node%20Object%20Reference) (ChildNode :type Card%20Node%20Object%20Reference))
  ;[0.15 0.15 0.15 0.5] Disconnect two nodes
  (if (and (Utilities|IsValid ParentNode) (Utilities|IsValid ChildNode))
    (bind (_errormsg _returnvalue) (Class|CardNode|BreakLinkwith ParentNode ChildNode))
    (if _returnvalue
      (Development|PrintText (Utilities|Text|FormatText (Utilities|Text|MakeLiteralText "{0} -> {1} is connected") (Class|Localisable|ToText ParentNode) (Class|Localisable|ToText ChildNode)))
      (else
        (Development|PrintText _errormsg true true "(R=1.000000,G=0.000000,B=0.000000,A=1.000000)")))))

(event Custom|Event%20On%20Connect%20Nodes
  (params (ParentNode :type Card%20Node%20Object%20Reference) (ChildNode :type Card%20Node%20Object%20Reference))
  ;[0.15 0.15 0.15 0.5] Connect two nodes
  (if (and (Utilities|IsValid ParentNode) (Utilities|IsValid ChildNode))
    (bind (_errormsg _returnvalue) (Class|CardNode|AddSuccessor ParentNode ChildNode))
    (if _returnvalue
      (Development|PrintText (Utilities|Text|FormatText (Utilities|Text|MakeLiteralText "{0} -> {1} is connected") (Class|Localisable|ToText ParentNode) (Class|Localisable|ToText ChildNode)))
      (else
        (Development|PrintText _errormsg true true "(R=1.000000,G=0.000000,B=0.000000,A=1.000000)")))))

(fn AddIngredient
  (params (Ingredient :type Card%20Ingredient%20Object%20Reference))
  (bind _returnvalue (Class|CardIngredient|WrapIntoNode Ingredient self))
  (return _returnvalue))

(fn GetCurrentRecipe
  (bind _owningplayer (Variables|Default|GetOwningPlayer))
  (bind _returnvalue (Game|ConstructObjectfromClass _owningplayer "/Game/Assets/Cards/Crafting/Recipe/BP_Recipe.BP_Recipe_C"))
  (bind _playerstate (Default|GetPlayerState _owningplayer))
  (bind _this (Default|CardNodetoRecipe _returnvalue (Variables|Default|GetCurrentRecipe) (Variables|/Game/Assets/Characters/Player/BP_DungeonSlayerPlayerState.BP_DungeonSlayerPlayerState_C|GetPlayerDeck _playerstate)))
  (return _this))