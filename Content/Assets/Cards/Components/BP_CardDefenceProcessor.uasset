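; BP_CardDefenceProcessor is a card component that applies the defence effects of a processed card to the character playing it.
; ProcessCard scans the card's effects for DefenceEffect entries and builds a GE_Defend spec from the source character's ability system.
; It passes each defence amount as a SetByCaller magnitude under the Defend combat tag, applies the spec to that same character, then prints the effect's text message.
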(event EventProcessCard
  (params (Card :type Card%20Object%20Reference) (SourceCharacter :type Basic%20Character%20Object%20Reference) (TargetCharacter :type Basic%20Character%20Object%20Reference))
  (bind _abilitysystemcomponent (Variables|/Script/CS3247_Project.BasicCharacter|GetAbilitySystemComponent SourceCharacter))
  (for _array_element (Variables|/Script/CS3247_Project.Card|GetEffects Card)
    (Utilities|IsValid (Class|CardEffect|GetEffect _array_element "/Script/CS3247_Project.DefenceEffect")
      (:Is%20Valid
        (bind _asdefence_effect (Utilities|Casting|CastToDefenceEffect (Class|CardEffect|GetEffect _array_element "/Script/CS3247_Project.DefenceEffect")))
        (bind _returnvalue (Ability|GameplayEffect|AssignTagSetbyCallerMagnitude (GameplayEffects|MakeOutgoingSpec :self _abilitysystemcomponent :GameplayEffectClass "/Game/Assets/GameplayAbilities/GameplayeEffects/GE_Defend.GE_Defend_C" :Level 1.0) "(TagName=\"GameplayEffect.Combat.Defend\")" (Math|Conversions|ToFloat(Integer) (Class|DefenceEffect|GetDefenceAmount _asdefence_effect))))
        (GameplayEffects|ApplyGameplayEffectSpecToTarget _abilitysystemcomponent _returnvalue _abilitysystemcomponent)
        (bind _returnvalue_2 (Class|Localisable|ToText(Message) _asdefence_effect))
        (Development|PrintText 0 _returnvalue_2)))))