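; BP_CardManaCostProcessor is a card component that charges a character mana when a card is processed.
; ProcessCard loops over the card's effects, picks out ManaCostEffect entries and reads their mana cost.
; Each cost becomes a SetByCaller magnitude on a GE_UseMana spec, applied to the character's own Ability System Component.
; It also prints each cost effect's text message.
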(event EventProcessCard
  (params (Card :type Card%20Object%20Reference) (Character :type Basic%20Character%20Object%20Reference))
  (bind _abilitysystemcomponent (Variables|/Script/CS3247_Project.BasicCharacter|GetAbilitySystemComponent Character))
  (for _array_element (Variables|/Script/CS3247_Project.Card|GetEffects Card)
    (bind _asmana_cost_effect (Utilities|Casting|CastToManaCostEffect (Class|CardEffect|GetEffect _array_element "/Script/CS3247_Project.ManaCostEffect")))
    (bind _returnvalue (Ability|GameplayEffect|AssignTagSetbyCallerMagnitude :SpecHandle (GameplayEffects|MakeOutgoingSpec :self _abilitysystemcomponent :GameplayEffectClass "/Game/Assets/GameplayAbilities/GameplayeEffects/GE_UseMana.GE_UseMana_C") :Magnitude (Math|Conversions|ToFloat(Integer) (Class|ManaCostEffect|GetManaCost _asmana_cost_effect))))
    (GameplayEffects|ApplyGameplayEffectSpecToSelf _abilitysystemcomponent _returnvalue)
    (bind _returnvalue_2 (Class|Localisable|ToText(Message) _asmana_cost_effect))
    (Development|PrintText 0 _returnvalue_2)))