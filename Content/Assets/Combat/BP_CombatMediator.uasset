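; Mediator actor that runs turn-based combat between the player and a list of enemies.
; BeginPlay wires combat, turn, action and death delegates, then starts combat and the player's turn.
; Enemies act sequentially with a combat context, stopping if the player dies, otherwise returning the turn.
; Actions apply Gameplay Ability System effects to self or target; dead enemies are destroyed, and combat ends when none remain.
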(event EventBeginPlay
  (EventDispatchers|BindEventtoOnCombatStarted (EventDispatchers|CreateEvent (Variables|Default|GetPlayer) :!event EventonEnterCombat))
  (EventDispatchers|BindEventtoOnCombatEnded (EventDispatchers|CreateEvent (Variables|Default|GetPlayer) :!event EventonExitCombat))
  (EventDispatchers|BindEventtoOnPlayerTurnStarted (EventDispatchers|CreateEvent (Variables|Default|GetPlayer) :!event EventonPlayerTurnStart))
  (EventDispatchers|BindEventtoOnPlayerTurnStarted (EventDispatchers|CreateEvent (Variables|Default|GetPlayer) :!event EventonPlayerTurnStart))
  ;[0.15 0.15 0.15 0.5] Turn Initialization
  (EventDispatchers|BindEventtoOnTurnEnded (Variables|Default|GetPlayer) (EventDispatchers|CreateEvent :!event Custom|Event%20On%20Start%20Enemy%20Turns))
  (EventDispatchers|BindEventtoOnCombatStarted (EventDispatchers|CreateEvent (Variables|Default|GetPlayer) :!event EventonEnterCombat))
  (for _array_element (Variables|Default|GetEnemies)
    (EventDispatchers|BindEventtoOnActionTaken _array_element (EventDispatchers|CreateEvent :!event Custom|Event%20On%20Execute%20Action))
    (EventDispatchers|BindEventtoOnDeath _array_element (EventDispatchers|CreateEvent :!event Custom|Event%20On%20Enemy%20Dead)))
  (Default|CallOnCombatStarted)
  (Default|CallOnPlayerTurnStarted))

(event Collision|EventActorBeginOverlap
  (params (OtherActor :type Actor%20Object%20Reference)))

(event EventTick
  (params (DeltaSeconds :type Float%20%28single-precision%29)))

(event Custom|Event%20On%20Enemy%20Dead
  (bind _enemies (Variables|Default|GetEnemies))
  (bind _deadenemies (CallFunction|FetchDeadEnemies))
  (for _array_element _deadenemies
    (Utilities|Array|RemoveItem _enemies _array_element)
    (Actor|DestroyActor _array_element))
  (if (Utilities|Array|IsEmpty _enemies)
    (Default|CallOnCombatEnded)))

(event Custom|Event%20On%20Execute%20Action
  (params (Target :type Basic%20Character%20Object%20Reference) (Instigator :type Basic%20Character%20Object%20Reference) (Level :type Float%20%28double-precision%29) (EffectDescriptor :type Gameplay%20Effect%20Descriptor%20Structure))
  (bind _spechandle (CallFunction|GenerateGameplayEffectSpec Instigator Level EffectDescriptor))
  (if (.bIsReflexive (Utilities|Struct|BreakGameplayEffectDescriptor EffectDescriptor))
    (GameplayEffects|ApplyGameplayEffectSpecToSelf (Variables|/Script/CS3247_Project.BasicCharacter|GetAbilitySystemComponent Instigator) _spechandle)
    (else
      (GameplayEffects|ApplyGameplayEffectSpecToTarget (Variables|/Script/CS3247_Project.BasicCharacter|GetAbilitySystemComponent Instigator) _spechandle (Variables|/Script/CS3247_Project.BasicCharacter|GetAbilitySystemComponent Target)))))

(event Custom|Event%20On%20Start%20Enemy%20Turns
  (bind _array_element (Utilities|Array|ForEachLoopwithBreak (Variables|Default|GetEnemies) :!label _label)
    (:LoopBody
      (Default|EventonTakeAction _array_element (Utilities|Struct|MakeCombatContext _array_element (Variables|Default|GetPlayer) (Variables|Default|GetEnemies)))
      (if (Variables|/Game/Assets/Characters/Player/BP_PlayerCharacter.BP_PlayerCharacter_C|GetIsDead (Variables|Default|GetPlayer))
        (Default|CallOnDeath (Variables|Default|GetPlayer))
        (goto _label Break)))
    (:Completed
      (if (not (Variables|/Game/Assets/Characters/Player/BP_PlayerCharacter.BP_PlayerCharacter_C|GetIsDead (Variables|Default|GetPlayer)))
        (Default|CallOnPlayerTurnStarted)
        (Audio|PlaySound2D "/Game/Audio/SFX/Combat/New_Turn_Cue.New_Turn_Cue" 1.0 1.0 0.0 0 0)))))

(fn ConstructionScript)

(fn FetchDeadEnemies
  (for _array_element (Variables|Default|GetEnemies)
    (if (Variables|/Game/Assets/Characters/Enemies/BP_EnemyCharacter.BP_EnemyCharacter_C|GetbIsDead _array_element)
      (Utilities|Array|AddUnique (LocalVariables|GetDead) _array_element)))
  (return (LocalVariables|GetDead)))