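; Turn manager Blueprint that runs turn-based combat between the player and a group of enemies.
; Combat start notifies the player, registers each enemy's death and attack events, and opens the player's turn.
; Ending that turn tells every enemy to act with an AI decision context, then immediately restarts the player's turn without waiting.
; Deaths trigger a winner check, which broadcasts the combat-ended event with the winning side.
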(event Custom|Event%20On%20Enemy%20Dead
  (params (DeadEnemy :type Enemy%20Character%20Object%20Reference))
  ;[0.15 0.15 0.15 0.5] Remove Dead Enemy
  (Utilities|Array|RemoveItem (Variables|Default|Getenemies) DeadEnemy)
  (bind _winner (CallFunction|CheckWinner))
  (switch Utilities|FlowControl|Switch|SwitchonE_CombatWinner _winner
    (:NewEnumerator0
      (CallFunction|EventonPlayerWin))
    (:NewEnumerator1
      (CallFunction|EventonEnemyWin))))

(event Custom|Event%20On%20Add%20Enemy
  (params (New%20Enemy :type BP%20Enemy%20Character%20Object%20Reference))
  (Utilities|Array|Add (Variables|Default|Getenemies) New%20Enemy)
  (EventDispatchers|BindEventtoOnEnemyDead New%20Enemy (delegate Custom|Event%20On%20Enemy%20Dead))
  (Development|PrintString (Utilities|String|Append (Utilities|GetDisplayName New%20Enemy) " entered battle scene!"))
  (EventDispatchers|BindEventtoOnEnemyAttacked New%20Enemy (EventDispatchers|CreateEvent (Variables|Player|GetPlayerCharacter) :!event EventonTakingDamage)))

(event Custom|RemoveEnemyFromTheArray
  (params (DeadEnemy :type Enemy%20Character%20Object%20Reference))
  ;[0.15 0.15 0.15 0.5] Remove Dead Enemy
  (Utilities|Array|RemoveItem (Variables|Default|Getenemies) DeadEnemy))

(event Custom|Event%20On%20Player%20Dead
  ;[0.15 0.15 0.15 0.5] Turn Initialization
  (bind _winner (CallFunction|CheckWinner))
  (switch Utilities|FlowControl|Switch|SwitchonE_CombatWinner _winner
    (:NewEnumerator0
      (Development|PrintString "A dead player won the battle..." true true "(R=1.000000,G=0.000000,B=0.000000,A=1.000000)"))
    (:NewEnumerator1
      (CallFunction|EventonEnemyWin))))

(event EventBeginPlay
  ;[0.15 0.15 0.15 0.5] Turn Initialization
  (bind _asbp_player_controller (Utilities|Casting|CastToBP_PlayerController (Pawn|GetController (Variables|Player|GetPlayerCharacter))))
  (bind _output_get (Variables|Player|SetPlayerController _asbp_player_controller))
  (Utilities|FlowControl|Delay 0.5)
  (EventDispatchers|BindEventtoOnPlayerTurnEnded _output_get (EventDispatchers|CreateEvent :!event Custom|Event%20On%20End%20Player%20Turn))
  (EventDispatchers|BindEventtoOnPlayerDead (Variables|Player|GetPlayerCharacter) (delegate Custom|Event%20On%20Player%20Dead))
  (EventDispatchers|BindEventtoOnCombatEnded (EventDispatchers|CreateEvent (Variables|Player|GetPlayerController) :!event EventonCombatEnd)))

(event Custom|Event%20On%20Enemy%20Win
  (Default|CallOnCombatEnded "NewEnumerator1"))

(event Custom|Event%20On%20Combat%20Start
  (params (Enemies :type Array%20of%20BP%20Enemy%20Character%20Object%20References))
  (Default|EventonCombatStart (Variables|Player|GetPlayerController))
  (Default|EventonCombatStart (Variables|Player|GetPlayerCharacter))
  (for _array_element Enemies
    (CallFunction|EventonAddEnemy _array_element))
  (CallFunction|EventonBeginPlayerTurn))

(event Custom|Event%20On%20End%20Player%20Turn
  ;[0.15 0.15 0.15 0.5] Event-On Player Turn End
  (for _array_element (Variables|Default|Getenemies)
    (bind _asbp_enemy_character (Utilities|Casting|CastToBP_EnemyCharacter _array_element))
    (Default|EventonTakeAction _asbp_enemy_character (Utilities|Struct|MakeAiDecisionContext _asbp_enemy_character (Variables|Player|GetPlayerCharacter))))
  (CallFunction|EventonBeginPlayerTurn))

(event Custom|Event%20On%20Begin%20Player%20Turn
  ;[0.15 0.15 0.15 0.5] Event-On Player Turn Begin
  (Default|EventonPlayerTurnStart (Variables|Player|GetPlayerController)))

(event Custom|Event%20On%20Player%20Win
  (Default|CallOnCombatEnded "NewEnumerator0"))

(event Custom|OnCombatEnd
  ;[0.15 0.15 0.15 0.5] Event-Combat End
  (if (Variables|/Game/Assets/Characters/Player/BP_PlayerCharacter.BP_PlayerCharacter_C|GetIsDead (Variables|Default|Getplayer))
    (Default|CallHideCombatHUD)
    (else
      (Widget|RemovefromParent (Variables|Default|GetturnUI))
      (Default|BattleEnd (Variables|Default|Getplayer))
      (Actor|DestroyActor))))

(fn ConstructionScript)

(fn CheckWinner
  (if (Utilities|Array|IsEmpty (Variables|Default|Getenemies))
    (return "NewEnumerator0")
    (elif (Variables|/Game/Assets/Characters/Player/BP_PlayerCharacter.BP_PlayerCharacter_C|GetIsDead (Variables|Player|GetPlayerCharacter))
      (return "NewEnumerator1")
      (else
        (return "NewEnumerator2")))))