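; Trigger zone that starts a combat encounter when the player character overlaps it, then destroys itself.
; On overlap, a timeline turns the player's view toward an anchor component while a weighted random pick selects a formation from the EnemyFormations data table.
; Enemies spawn evenly spaced between two anchors generated from the player's position, then pass with the player to a spawned BP_CombatMediator.
; OnEnable turns on the trigger's overlap events.
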(event OnComponentBeginOverlap(TriggerZone)
  (params (OverlappedComponent :type Primitive%20Component%20Object%20Reference) (OtherActor :type Actor%20Object%20Reference) (OtherComp :type Primitive%20Component%20Object%20Reference) (OtherBodyIndex :type Integer) (bFromSweep :type Boolean) (SweepResult :type Hit%20Result%20Structure%20%28by%20ref%29))
  ;[0.15 0.15 0.15 0.5] Spawn Enemies and TurnManager
  (bind _asbp_player_character (Utilities|Casting|CastToBP_PlayerCharacter OtherActor))
  (bind _output_get (Variables|Default|SetPlayerCharacter _asbp_player_character))
  (CallFunction|AdjustCamera)
  (Utilities|FlowControl|Delay 0.2)
  (bind _enemies_to_spawn (CallFunction|SelectEnemies))
  (bind _enemycharacters (CallFunction|SpawnEnemies _enemies_to_spawn))
  (Game|SpawnActorfromClass "/Game/Assets/Combat/BP_CombatMediator.BP_CombatMediator_C" (Transformation|GetActorTransform self) "AlwaysSpawn" "MultiplyWithRoot" 0 _output_get _enemycharacters 0)
  (Audio|PlaySoundatLocation "/Game/Audio/SFX/Combat/Enemy_Spawning.Enemy_Spawning" (Transformation|GetActorLocation) "0, 0, 0" 1.0 1.0 0.0 0 0 self 0)
  (Actor|DestroyActor))

(event Custom|Event%20On%20Enable
  (Variables|/Script/Engine.PrimitiveComponent|SetbGenerateOverlapEvents (Variables|Default|GetTriggerZone) true))

(event EventBeginPlay
  (bind _outrownames (DataTable|GetDataTableRowNames (Variables|Default|GetEnemyFormations)))
  (for _array_element _outrownames
    (bind _returnvalue (Utilities|GetDataTableRow (Variables|Default|GetEnemyFormations) _array_element)
      (:then
        (Variables|EnemySpawning|SetTotalWeight (+ (.Weight (Utilities|Struct|BreakS_EnemyFormationRowStructure _returnvalue)) (Variables|EnemySpawning|GetTotalWeight)))))))

(event Custom|Adjust%20Camera
  (bind _speed (Timeline|rotation Play)
    (:Update
      (Pawn|SetControlRotation (Pawn|GetController (Variables|Default|GetPlayerCharacter)) (Math|Rotator|Lerp(Rotator) (Math|Rotator|MakeRotator 0.0 0.0 (.Yaw (Math|Rotator|BreakRotator (Math|Rotator|FindLookatRotation (Transformation|GetActorLocation (Variables|Default|GetPlayerCharacter)) (Transformation|GetWorldLocation (Variables|Default|GetAnker)))))) "0, 0, 0" _speed)))))

(fn ConstructionScript)

(fn SelectEnemies
  (LocalVariables|SetIndex (Math|Random|RandomIntegerinRange 1 (Variables|EnemySpawning|GetTotalWeight)))
  (bind _outrownames (DataTable|GetDataTableRowNames (Variables|Default|GetEnemyFormations)))
  (for _array_element _outrownames
    (bind _returnvalue (Utilities|GetDataTableRow (Variables|Default|GetEnemyFormations) _array_element)
      (:then
        (bind _output_get (LocalVariables|SetCumulativeWeight (+ (.Weight (Utilities|Struct|BreakS_EnemyFormationRowStructure _returnvalue)) (LocalVariables|GetCumulativeWeight))))
        (if (>= _output_get (LocalVariables|GetIndex))
          (return (.Enemies (Utilities|Struct|BreakS_EnemyFormationRowStructure _returnvalue))))))))

(fn FindSpawnTransform
  (params (NumberOfEnemies :type Integer) (CurrentEnemyIndex :type Integer) (Anker1Loc :type Vector) (Anker2Loc :type Vector))
  (return (Math|Conversions|ToTransform(Vector) (+ (* (+ CurrentEnemyIndex 1) (/ (- Anker1Loc Anker2Loc) (+ NumberOfEnemies 1))) Anker2Loc))))

(fn SpawnEnemies
  (params (EnemyData :type Array%20of%20Enemy%20Object%20References))
  (for (_array_element _array_index) EnemyData
    (bind (_anchor1 _anchor2) (CallFunction|FindTwoAnkers))
    (bind _spawn_transform (CallFunction|FindSpawnTransform (Utilities|Array|Length EnemyData) _array_index _anchor1 _anchor2))
    (bind _returnvalue (Game|SpawnActorfromClass "/Game/Assets/Characters/Enemies/BP_EnemyCharacter.BP_EnemyCharacter_C" _spawn_transform "Undefined" "MultiplyWithRoot" 0 _array_element 0))
    (Utilities|Array|Add (LocalVariables|GetSpawnedEnemies) _returnvalue)
    (Transformation|SetActorRotation _returnvalue (Math|Rotator|FindLookatRotation (Transformation|GetActorLocation (Variables|Default|GetPlayerCharacter)) (Transformation|GetActorLocation _returnvalue))))
  (return (LocalVariables|GetSpawnedEnemies)))

(fn FindTwoAnkers
  (bind _returnvalue (Class|GenerateEnemySpawnAnchors|GenerateAnchorsBasedonPlayer (Variables|Default|GetPlayerCharacter) 5e+02 4e+02))
  (return (Utilities|Array|Get(acopy) _returnvalue) (Utilities|Array|Get(acopy) _returnvalue 1)))