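; Actor component that runs slide and hard-landing actions for BP_GameplayPlayer, caching the player character on BeginPlay.
; Sliding plays a running-slide montage behind a DoOnce that resets after a short cooldown once the montage completes.
; HardLand checks vertical fall speed, then plays a landing montage and voice sound while briefly disabling input and camera pawn-control rotation through helper events.
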(event Custom|Sliding
  (params (Enable%20Slide :type Boolean))
  ;[0 0.15 0.007331 0.5] Slide Function
  (if Enable%20Slide
    (Utilities|FlowControl|DoOnce false :!label _label
      (:Completed
        (Animation|Montage|PlayMontage (Variables|/Script/Engine.Character|GetMesh (Variables|PlayerReference|GetAs%20BP%20Gameplay%20Player)) "/Game/Assets/TFPMovement/CHARACTER/Animations/Locomotion/Action/Montage/AS_ALSv2_N_RunningSlide_UE_Montage.AS_ALSv2_N_RunningSlide_UE_Montage"
          (:OnCompleted
            (Utilities|FlowControl|Delay 1.0 :!pinned true) ; Delay when you can slide again
            (goto _label Reset)))))))

(event Custom|Enable/Disable%20Input%20function
  (params (Disable%20Input :type Boolean))
  (bind _returnvalue (Game|GetPlayerController 0))
  (bind _as_bp_gameplay_player (Variables|PlayerReference|GetAs%20BP%20Gameplay%20Player))
  ;[0 0.15 0.007331 0.5] Disable/Enable Input
  (if Disable%20Input
    (Input|DisableInput _as_bp_gameplay_player _returnvalue)
    (else
      (Input|EnableInput _as_bp_gameplay_player _returnvalue))))

(event Custom|HardLand
  (params (Enable%20HardLand :type Boolean))
  ;[0 0.15 0.007331 0.5] HardLand Function
  (if Enable%20HardLand
    (if (Math|Float|InRange(Float) (Math|Float|Absolute(Float) (.Z (Math|Vector|BreakVector (Variables|/Script/Engine.MovementComponent|GetVelocity (Variables|/Script/Engine.Character|GetCharacterMovement (Variables|PlayerReference|GetAs%20BP%20Gameplay%20Player)))))) 6.5e+02 5e+03)
      (CallFunction|Enable/DisableInputFunction true)
      (CallFunction|SetPawnControl false)
      (Animation|PlayAnimMontage (Variables|PlayerReference|GetAs%20BP%20Gameplay%20Player) "/Game/Assets/TFPMovement/CHARACTER/Animations/Locomotion/Action/Montage/AS_ALS_MediumLand_Forward_Montage.AS_ALS_MediumLand_Forward_Montage" 1.0 "None")
      ;;[0.009248 0.15 0 0.5] [EXAMPLE] Play HardLand Voice SFX
      (Audio|SpawnSoundAttached "/Game/Assets/TFPMovement/AUDIO/Character/Voice/SoundCues/Voice_Land_Cue.Voice_Land_Cue" (Variables|/Script/Engine.Character|GetMesh (Variables|PlayerReference|GetAs%20BP%20Gameplay%20Player)) "None" "0, 0, 0" "0, 0, 0" "KeepRelativeOffset" false 1.0 1.0 0.0 "/Game/Assets/TFPMovement/AUDIO/Character/Voice/SA_VoiceSoundAttenuation.SA_VoiceSoundAttenuation" 0)
      (Utilities|FlowControl|Delay 1.35)
      (CallFunction|Enable/DisableInputFunction false)
      (CallFunction|SetPawnControl true))))

(event Custom|SetPawnControl
  (params (ON :type Boolean))
  (bind _as_bp_gameplay_player (Variables|PlayerReference|GetAs%20BP%20Gameplay%20Player))
  (bind _fpscamera (Variables|/Game/Assets/TFPMovement/BLUEPRINT/Player/BP_GameplayPlayer.BP_GameplayPlayer_C|GetFPSCamera _as_bp_gameplay_player))
  ;[0 0.15 0.007331 0.5] Disable/Enable Pawn Control Rotation
  (if ON
    (Variables|/Script/Engine.CameraComponent|SetbUsePawnControlRotation _fpscamera true)
    (else
      (Variables|/Script/Engine.CameraComponent|SetbUsePawnControlRotation _fpscamera false))))

(event EventBeginPlay
  ;[0 0.02129 0.15 0.5] Cast to Player
  (bind _asbp_gameplay_player (Utilities|Casting|CastToBP_GameplayPlayer (Game|GetPlayerCharacter 0)))
  (Variables|PlayerReference|SetAs%20BP%20Gameplay%20Player _asbp_gameplay_player))