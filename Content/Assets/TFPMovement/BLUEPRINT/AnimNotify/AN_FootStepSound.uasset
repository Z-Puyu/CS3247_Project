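; Animation notify that plays surface-dependent footstep audio on the player character.
; It gets the player from the mesh owner through GetPlayerMessage and traces a short distance down from the foot socket chosen by RightFoot.
; The hit physical material is looked up in PhysicMat and sent as the "floor" integer parameter to the audio component.
; The Moving and Jump flags select that component, with SCFootSteps used for movement.
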(fn ReceivedNotify
  (params (MeshComp :type Skeletal%20Mesh%20Component%20Object%20Reference) (Animation :type Anim%20Sequence%20Base%20Object%20Reference) (EventReference :type Anim%20Notify%20Event%20Reference%20Structure%20%28by%20ref%29))
  (bind _player (Class|BPIPlayerReference|GetPlayer(Message) (Components|GetOwner MeshComp)))
  (LocalVariables|SetPlayer _player)
  (bind _outhit (Collision|LineTraceByChannel (Transformation|GetSocketLocation (Variables|/Script/Engine.Character|GetMesh (LocalVariables|GetPlayer)) (select (Variables|Default|GetRightFoot?) "foot_r" "foot_l")) (- (Transformation|GetSocketLocation (Variables|/Script/Engine.Character|GetMesh (LocalVariables|GetPlayer)) (select (Variables|Default|GetRightFoot?) "foot_r" "foot_l")) "0,0,50.000000") "TraceTypeQuery1" false (Utilities|Array|MakeArray (Components|GetOwner MeshComp)) "None"))
  (Audio|Components|Audio|Play (select (Variables|Default|GetMoving?) (Variables|/Game/Assets/TFPMovement/BLUEPRINT/Player/BP_GameplayPlayer.BP_GameplayPlayer_C|GetSC_FootSteps (LocalVariables|GetPlayer)) (select (Variables|Default|GetJump?) 0 0)) 0.0)
  (Effects|Components|ParticleSystem|SetIntParameter (select (Variables|Default|GetMoving?) (Variables|/Game/Assets/TFPMovement/BLUEPRINT/Player/BP_GameplayPlayer.BP_GameplayPlayer_C|GetSC_FootSteps (LocalVariables|GetPlayer)) (select (Variables|Default|GetJump?) 0 0)) "floor" (Utilities|Array|FindItem (Variables|Default|GetPhysicMat) (.PhysMat (Collision|BreakHitResult _outhit))))
  (return true))