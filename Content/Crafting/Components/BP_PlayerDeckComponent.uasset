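; Player deck component that stores the player's cards in a map and provides random draws from it.
; AddCard keys each entry by the card, with a card structure built from its name and description.
; RandomDraw returns a random key without removing it from the deck.
; ConnectEvents binds to a card crafter's OnCardCrafted event, intended to add newly crafted cards.
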(fn RandomDraw
  (bind _keys (Utilities|Map|Keys (Variables|Default|GetCards)))
  (return (.OutItem (Utilities|Array|Random _keys))))

(fn AddCard
  (params (Card :type Card%20Object%20Reference))
  (bind (_cardname _desc) (Class|Card|GetCardInfo Card))
  (Utilities|Map|Add (Variables|Default|GetCards) Card (Utilities|Struct|MakeS_CardStructure "00000000000000000000000000000000" _cardname 0 _desc)))

(fn ConnectEvents
  (params (CardCrafter :type BP%20Card%20Crafter%20Component%20Object%20Reference))
  (Events|AddCardonNewCardCrafted CardCrafter))

(fn AddCardonNewCardCrafted
  (params (Card%20Crafter :type BP%20Card%20Crafter%20Component%20Object%20Reference))
  (EventDispatchers|BindEventtoOnCardCrafted Card%20Crafter (EventDispatchers|CreateEvent :!event AddCard)))