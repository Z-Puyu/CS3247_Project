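; Card crafting component that tracks ingredient nodes and builds a new card from their connected graph.
; Adding or removing a node revalidates the recipe, which passes only when the buildable connected node count equals the total, and broadcasts the result.
; Crafting builds effects from the root node, constructs and broadcasts the Card, then clears the nodes.
; ConnectUIEvents binds the crafting area, ingredient list and craft button to these events.
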(fn MakeCard
  (params (CardName :type Text) (UseCost :type Integer) (CardDurability :type Integer) (CardEffects :type Array%20of%20Card%20Effect%20Object%20References))
  (bind _returnvalue (Game|ConstructObjectfromClass "/Script/CS3247_Project.Card" CardName UseCost CardDurability CardEffects))
  (return _returnvalue))

(fn AddIngredient
  (params (Node :type Card%20Node%20Object%20Reference))
  (Utilities|Set|Add (Variables|Default|GetNodes) Node)
  (bind _bisbuildable (CallFunction|ValidateRecipe Node))
  (if _bisbuildable
    (Development|PrintString "Ready to Craft!")
    (else
      (Development|PrintString "Recipe not Valid!")))
  (Default|CallOnRecipeChanged _bisbuildable))

(fn ConnectUIEvents
  (params (Crafting%20Area%20UI :type WBP%20Crafting%20Area%20Object%20Reference) (Ingredient%20List%20UI :type WBP%20List%20Of%20Ingredients%20Object%20Reference) (Craft%20Button%20UI :type Button%20Object%20Reference))
  (UIEvents|AddCardNodeonNewIngredient Crafting%20Area%20UI)
  (UIEvents|ClearCraftingAreaonNewCardCrafted Crafting%20Area%20UI)
  (UIEvents|RemoveCardNodeonWithdrawingIngredient Ingredient%20List%20UI)
  (UIEvents|ToggleCraftButtonHitDetectiononRecipeChanged Craft%20Button%20UI)
  (UIEvents|CraftCardonCraftButtonClicked Craft%20Button%20UI))

(fn RemoveIngredient
  (params (DeletedNode :type Card%20Node%20Object%20Reference))
  (bind _nodes (Variables|Default|GetNodes))
  (bind _returnvalue (Utilities|Set|Remove (Variables|Default|GetNodes) DeletedNode))
  (if _returnvalue
    (Development|PrintText (Utilities|Text|FormatText (Utilities|Text|MakeLiteralText "Removed {0}") (Variables|/Script/CS3247_Project.CardIngredient|GetName (Variables|/Script/CS3247_Project.CardNode|GetIngredient DeletedNode))))
    (if (Utilities|Set|IsEmpty _nodes)
      (Default|CallOnRecipeChanged false)
      (else
        (bind _result (Utilities|Set|ToArray _nodes))
        (bind _bisbuildable (CallFunction|ValidateRecipe (Utilities|Array|Get(acopy) _result)))
        (Default|CallOnRecipeChanged _bisbuildable)))
    (else
      (Development|PrintString "Removing non-existent ingredient!" true true "(R=1.000000,G=0.000000,B=0.000000,A=1.000000)"))))

(fn ValidateRecipe
  (params (Source :type Card%20Node%20Object%20Reference))
  (bind _returnvalue (Class|CardNode|CountBuildableConnectedNodes Source))
  (Development|PrintText (Utilities|Text|FormatText (Utilities|Text|MakeLiteralText "{0} buildable nodes") _returnvalue))
  (return (== _returnvalue (Utilities|Set|Length (Variables|Default|GetNodes)))))

(fn CraftNewCard
  (bind _nodes (Variables|Default|GetNodes))
  (bind _result (Utilities|Set|ToArray _nodes))
  (bind _returnvalue (Class|CardNode|GetRoot (Utilities|Array|Get(acopy) _result)))
  (bind _returnvalue_2 (Class|CardNode|Build _returnvalue))
  (bind _new_card (CallFunction|MakeCard "New Card" 0 0 _returnvalue_2))
  (Default|CallOnCardCrafted _new_card)
  (Utilities|Set|Clear _nodes)
  (Development|PrintString "New card crafted!"))

(fn ClearCraftingAreaonNewCardCrafted
  (params (CraftingAreaUI :type WBP%20Crafting%20Area%20Object%20Reference))
  (EventDispatchers|BindEventtoOnCardCrafted (EventDispatchers|CreateEvent CraftingAreaUI :!event CompleteCrafting)))

(fn AddCardNodeonNewIngredient
  (params (CraftingAreaUI :type WBP%20Crafting%20Area%20Object%20Reference))
  (EventDispatchers|BindEventtoOnNewIngredientAdded CraftingAreaUI (EventDispatchers|CreateEvent :!event AddIngredient)))

(fn RemoveCardNodeonWithdrawingIngredient
  (params (IngredientListUI :type WBP%20List%20Of%20Ingredients%20Object%20Reference))
  (EventDispatchers|BindEventtoOnIngredientWithdrawn IngredientListUI (EventDispatchers|CreateEvent :!event RemoveIngredient)))

(fn ToggleCraftButtonHitDetectiononRecipeChanged
  (params (CraftButtonUI :type Button%20Object%20Reference))
  (EventDispatchers|BindEventtoOnRecipeChanged (EventDispatchers|CreateEvent CraftButtonUI :!event SetIsEnabled)))

(fn CraftCardonCraftButtonClicked
  (params (CraftButtonUI :type Button%20Object%20Reference))
  (EventDispatchers|BindEventtoOnClicked CraftButtonUI (EventDispatchers|CreateEvent :!event CraftNewCard)))